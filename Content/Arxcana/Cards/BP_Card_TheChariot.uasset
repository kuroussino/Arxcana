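; The Chariot tarot card, which lets the player preview and place a cement block in the world.
; Entering the hand disables its box collision and turns on the guide.
; While active, a delay-throttled Tick traces from the camera to spawn, move or remove the guide at the hit point.
; PlaceBlock, not called within this Blueprint, swaps a legally positioned guide for a block, replacing any previously placed one.
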(event EventBeginPlay
  (|CallParentFunction)
  (Variables|Default|SetCardType "NewEnumerator2"))

(event Collision|EventActorBeginOverlap
  (params (OtherActor :type Actor%20Object%20Reference))
  (|CallParentFunction OtherActor) ; This node is disabled and will not be called.\nDrag off pins to build functionality.
)

(event EventTick
  (params (DeltaSeconds :type Float%20%28single-precision%29))
  (|CallParentFunction DeltaSeconds)
  (if (Variables|Default|GetisActive)
    (Utilities|FlowControl|Delay 0.025)
    (if (Variables|Default|GetneedShowGuide)
      (CallFunction|ShowGuide)
      (elif (Utilities|IsValid (Variables|Default|GetcurrGuide))
        (CallFunction|DestroyGuide)))))

(event EventDestroyed
  (CallFunction|DestroyGuide))

(event EventInHand/NotinHand
  (params (Enabled/Disabled :type Boolean))
  (|CallParentFunction Enabled/Disabled)
  (if Enabled/Disabled
    (Collision|SetCollisionEnabled (Variables|Default|GetBox) "NoCollision")
    (CallFunction|ToggleFunction)))

(fn ConstructionScript
  (|CallParentFunction))

(fn ToggleFunction
  (Variables|Default|SetneedShowGuide true))

(fn ShowGuide
  (bind _returnvalue (Game|GetPlayerCameraManager 0))
  (bind _returnvalue_2 (Game|GetPlayerCameraManager 0))
  (bind _returnvalue_3 (Camera|GetCameraLocation _returnvalue))
  (bind _returnvalue_4 (Camera|GetCameraLocation _returnvalue_2))
  (if (Utilities|IsValid (Variables|Default|GetcurrGuide))
    (bind (_outhit _returnvalue_5) (Collision|LineTraceByChannel _returnvalue_3 (+ _returnvalue_3 (* (Math|Vector|GetForwardVector (Camera|GetCameraRotation _returnvalue)) (Variables|Default|GetlineTraceDistance))) "TraceTypeQuery1" false (Utilities|Array|MakeArray (Variables|Default|GetcurrGuide)) "None"))
    (if _returnvalue_5
      (Transformation|SetActorLocation (Variables|Default|GetcurrGuide) (.Location (Collision|BreakHitResult _outhit)) false false)
      (else
        (Actor|DestroyActor (Variables|Default|GetcurrGuide))
        (Variables|Default|SetcurrGuide 0)))
    (else
      (bind (_outhit_2 _returnvalue_6) (Collision|LineTraceByChannel _returnvalue_4 (+ _returnvalue_4 (* (Math|Vector|GetForwardVector (Camera|GetCameraRotation _returnvalue_2)) (Variables|Default|GetlineTraceDistance))) "TraceTypeQuery1" false 0 "None"))
      (if _returnvalue_6
        (bind _returnvalue_7 (Game|SpawnActorfromClass "/Game/Arxcana/Placeables/BP_CementBlockGuide.BP_CementBlockGuide_C" (Math|Conversions|ToTransform(Vector) (.Location (Collision|BreakHitResult _outhit_2))) "Undefined" "MultiplyWithRoot" 0 0))
        (Variables|Default|SetcurrGuide _returnvalue_7)))))

(fn PlaceBlock
  (if (Utilities|IsValid (Variables|Default|GetcurrGuide))
    (if (Variables|/Game/Arxcana/Placeables/BP_CementBlockGuide.BP_CementBlockGuide_C|GetlegalPosition (Variables|Default|GetcurrGuide))
      (bind _returnvalue (Game|SpawnActorfromClass "/Game/Arxcana/Placeables/BP_CementBlock.BP_CementBlock_C" (Transformation|GetActorTransform (Variables|Default|GetcurrGuide)) "AdjustIfPossibleButAlwaysSpawn" "MultiplyWithRoot" 0 0))
      (if (Utilities|IsValid (Variables|Default|GetplacedBlock))
        (Actor|DestroyActor (Variables|Default|GetplacedBlock))
        (Variables|Default|SetplacedBlock _returnvalue)
        (else
          (Variables|Default|SetplacedBlock _returnvalue)))
      (Actor|DestroyActor (Variables|Default|GetcurrGuide))
      (Variables|Default|SetcurrGuide 0))))

(fn DestroyGuide
  (Utilities|IsValid (Variables|Default|GetcurrGuide)
    (:Is%20Valid
      (Actor|DestroyActor (Variables|Default|GetcurrGuide))
      (Variables|Default|SetcurrGuide 0))))