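; The High Priestess card, a child card Blueprint that flips the world between two global states, A and B.
; ToggleFunction puts affected BP_SwitchableObjects into or out of a changing state, passing the current state and yellow/red editing materials on entry.
; SwitchState flips GlobalState on BP_MainCharacter, then sends the new state to each affected actor through SwitchStateMessage.
; BeginPlay sets the card type, while other events defer to the parent.
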(event EventBeginPlay
  (|CallParentFunction)
  (Variables|Default|SetCardType "NewEnumerator4"))

(event Collision|EventActorBeginOverlap
  (params (OtherActor :type Actor%20Object%20Reference))
  (|CallParentFunction OtherActor) ; This node is disabled and will not be called.\nDrag off pins to build functionality.
)

(event EventTick
  (params (DeltaSeconds :type Float%20%28single-precision%29))
  (|CallParentFunction DeltaSeconds))

(event EventInHand/NotinHand
  (params (Enabled/Disabled :type Boolean))
  (|CallParentFunction Enabled/Disabled))

(fn ConstructionScript
  (|CallParentFunction))

(fn ToggleFunction
  (params (enabling/Disabling :type Boolean) (affectedActors :type Array%20of%20Actor%20Object%20References) (globalState :type BPE_HighPriestressState%20Enum :default "NewEnumerator0"))
  (if enabling/Disabling
    (for _array_element affectedActors
      (bind _asbp_switchable_object (Utilities|Casting|CastToBP_SwitchableObject _array_element))
      (Default|EnterChangingState _asbp_switchable_object globalState "/Game/Debug/MaterialLibrary/MM_Editing2_Yellow.MM_Editing2_Yellow" "/Game/Debug/MaterialLibrary/MM_Editing2_Red.MM_Editing2_Red"))
    (else
      (for _array_element_2 affectedActors
        (bind _asbp_switchable_object_2 (Utilities|Casting|CastToBP_SwitchableObject _array_element_2))
        (Default|ExitChangingState _asbp_switchable_object_2 globalState)))))

(fn SwitchState
  (params (affectedActors :type Array%20of%20Actor%20Object%20References) (globalState :type BPE_HighPriestressState%20Enum :default "NewEnumerator0"))
  (switch Utilities|FlowControl|Switch|SwitchonBPE_HighPriestressState globalState
    (:NewEnumerator0
      (bind _asbp_main_character (Utilities|Casting|CastToBP_MainCharacter (Game|GetPlayerCharacter 0)))
      (bind _output_get (Variables|/Game/Arxcana/Core/MainCharacter/BP_MainCharacter.BP_MainCharacter_C|SetglobalState _asbp_main_character "NewEnumerator1"))
      (Development|PrintString "Switched to state B")
      (for _array_element affectedActors
        (Class|BPISwitchable|SwitchState(Message) _array_element _output_get)))
    (:NewEnumerator1
      (bind _asbp_main_character_2 (Utilities|Casting|CastToBP_MainCharacter (Game|GetPlayerCharacter 0)))
      (bind _output_get_2 (Variables|/Game/Arxcana/Core/MainCharacter/BP_MainCharacter.BP_MainCharacter_C|SetglobalState _asbp_main_character_2 "NewEnumerator0"))
      (Development|PrintString "Switched to state A")
      (for _array_element_2 affectedActors
        (Class|BPISwitchable|SwitchState(Message) _array_element_2 _output_get_2)))))