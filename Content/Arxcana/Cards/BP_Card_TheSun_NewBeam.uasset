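; The Sun card, a card Blueprint whose ability is a laser beam, with a point light that switches on when the card is in hand.
; ToggleFunction spawns a laser emitter at BeamStart aimed along the player camera, attaches it and starts it emitting, or stops and destroys it.
; If the card is destroyed while active, it shuts off both beam and light.
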(event EventBeginPlay
  (|CallParentFunction)
  (Variables|Default|SetCardType "NewEnumerator0"))

(event EventTick
  (params (DeltaSeconds :type Float%20%28single-precision%29))
  (|CallParentFunction DeltaSeconds))

(event EventInHand/NotinHand
  (params (Enabled/Disabled :type Boolean))
  (|CallParentFunction Enabled/Disabled)
  (if Enabled/Disabled
    (CallFunction|SetFlashlightVisibility true)))

(event EventDestroyed
  (if (Variables|Default|GetisActive)
    (CallFunction|ToggleFunction false)
    (CallFunction|SetFlashlightVisibility false)))

(fn ConstructionScript
  (|CallParentFunction))

(fn SetFlashlightVisibility
  (params (active :type Boolean))
  (bind _pointlight (Variables|Default|GetPointLight))
  (if active
    (Rendering|SetVisibility _pointlight true false)
    (else
      (Rendering|SetVisibility _pointlight false false))))

(fn ToggleFunction
  (params (beam :type Boolean))
  (bind _beamstart (Variables|Default|GetBeamStart))
  (if beam
    (bind _returnvalue (Game|SpawnActorfromClass "/Game/Arxcana/Core/LaserSystem/BP_LaserEmitter_Card_TheSun_NewBeam.BP_LaserEmitter_Card_TheSun_NewBeam_C" (Math|Transform|MakeTransform (Transformation|GetWorldLocation _beamstart) (Camera|GetCameraRotation (Game|GetPlayerCameraManager 0)) "1.000000,1.000000,1.000000") "Undefined" "MultiplyWithRoot" 0 0))
    (bind _output_get (Variables|Default|SetcurrentBeam _returnvalue))
    (Transformation|AttachComponentToComponent _output_get _beamstart "None" "KeepWorld" "KeepWorld" "KeepWorld" true)
    (Variables|/Game/Arxcana/Core/LaserSystem/BP_LaserEmitter_Card_TheSun_NewBeam.BP_LaserEmitter_Card_TheSun_NewBeam_C|Setemitting (Variables|Default|GetcurrentBeam) true)
    (else
      (Utilities|IsValid (Variables|Default|GetcurrentBeam)
        (:Is%20Valid
          (Default|StopBeam (Variables|Default|GetcurrentBeam))
          (Variables|/Game/Arxcana/Core/LaserSystem/BP_LaserEmitter_Card_TheSun_NewBeam.BP_LaserEmitter_Card_TheSun_NewBeam_C|Setemitting (Variables|Default|GetcurrentBeam) false)
          (Actor|DestroyActor (Variables|Default|GetcurrentBeam))
          (Variables|Default|SetcurrentBeam 0))))))