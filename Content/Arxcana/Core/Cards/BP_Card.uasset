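; BP_Card is a card actor that turns to face the player's camera while it is not held in a hand.
; Each Tick it interpolates its yaw toward the look-at rotation to the first player's camera, setting only yaw for a smooth billboard effect.
; SetHolding toggles the IsInHand flag that suspends this facing, and Destroyed clears it.
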(event EventTick
  (params (DeltaSeconds :type Float%20%28single-precision%29))
  (if (not (Variables|Default|GetisInHand))
    (Transformation|SetActorRotation (Math|Rotator|MakeRotator 0.0 0.0 (.yaw (Math|Interpolation|RInterpTo (Transformation|GetActorRotation) (Math|Rotator|FindLookatRotation (Transformation|GetActorLocation) (Camera|GetCameraLocation (Game|GetPlayerCameraManager 0))) (Utilities|Time|GetWorldDeltaSeconds) 7.5))))))

(event EventSetHolding
  (params (Holding :type Boolean))
  (Variables|Default|SetisInHand Holding))

(event EventDestroyed
  (Variables|Default|SetisInHand false))

(fn ConstructionScript)