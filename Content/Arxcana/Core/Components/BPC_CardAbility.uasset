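; BPC_CardAbility is an actor component that serves as a skeleton for card abilities.
; On begin play it casts player 0's character to BP_MainCharacter and sets its CardInHand to holding, logging the attachment; end play logs the component name and reason.
; TogglePrimaryAbility and ToggleSecundaryAbility take a pressed/released input and player reference but are empty here.
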(event EventBeginPlay
  (Development|PrintString (Utilities|String|Append "Component attached: " (Utilities|GetObjectName self)))
  (bind _asbp_main_character (Utilities|Casting|CastToBP_MainCharacter (Game|GetPlayerCharacter 0)))
  (Default|SetHolding (Variables|/Game/Arxcana/Core/MainCharacter/BP_MainCharacter.BP_MainCharacter_C|GetcardInHand _asbp_main_character) true))

(event EventEndPlay
  (params (EndPlayReason :type EEndPlayReason%20Enum :default "Destroyed"))
  ;[1 0.01578 0] Debug
  (Development|PrintString (Utilities|String|Append "component named " (Utilities|GetObjectName self) " ended for reason:" (Utilities|String|EnumtoString EndPlayReason))))

(fn TogglePrimaryAbility
  (params (pressed/Released :type Boolean) (playerRef :type BP%20Main%20Character%20Object%20Reference)))

(fn ToggleSecundaryAbility
  (params (pressed/Released :type Boolean) (playerRef :type BP%20Main%20Character%20Object%20Reference)))