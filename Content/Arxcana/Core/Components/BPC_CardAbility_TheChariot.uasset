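; Card ability component for The Chariot card, letting the player place blocks with the primary ability.
; On press, the primary toggle runs the parent logic, then casts the player's card in hand to BP_Card_TheChariot and calls PlaceBlock.
; The secondary toggle only calls its parent, as its DestroyCurrentBlock logic is disconnected and never runs.
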(event EventBeginPlay)

(event EventTick
  (params (DeltaSeconds :type Float%20%28single-precision%29)))

(fn TogglePrimaryAbility
  (params (pressed/Released :type Boolean) (playerRef :type BP%20Main%20Character%20Object%20Reference))
  (|CallParentFunction pressed/Released playerRef)
  (if pressed/Released
    (bind _asbp_card_the_chariot (Utilities|Casting|CastToBP_Card_TheChariot (Variables|/Game/Arxcana/Core/MainCharacter/BP_MainCharacter.BP_MainCharacter_C|GetcardInHand playerRef)))
    (Default|PlaceBlock _asbp_card_the_chariot)))

(fn ToggleSecundaryAbility
  (params (pressed/Released :type Boolean) (playerRef :type BP%20Main%20Character%20Object%20Reference))
  (|CallParentFunction pressed/Released playerRef))