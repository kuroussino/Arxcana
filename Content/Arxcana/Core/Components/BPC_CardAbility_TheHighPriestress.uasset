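; High Priestess card ability component that flips switchable objects in the player's current switch area between two states, A and B.
; On BeginPlay a small sphere overlap at the player finds a BP_SwitchArea, caches its state and objects, and puts them into a changing state with a fog material.
; Primary press toggles the state and messages each object.
; EndPlay exits the changing state and saves the state back to the area.
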(event EventBeginPlay
  (bind _found (CallFunction|FindSwitchArea))
  (if _found
    (Development|PrintString "Switch area found!")
    (CallFunction|ToggleSwitchState true)
    (Variables|Default|Setin%20changing%20state true)
    (else
      (Development|PrintString "Switch area not found!"))))

(event EventEndPlay
  (params (EndPlayReason :type EEndPlayReason%20Enum :default "Destroyed"))
  (CallFunction|ResetHighPriestress)
  (bind _currswitcharea (Variables|Default|GetcurrSwitchArea)
    (:then
      (bind _output_get (Variables|/Game/Arxcana/Core/SwitchableObjects/BP_SwitchArea.BP_SwitchArea_C|SetareaState _currswitcharea (Variables|Default|GetglobalState)))
      (CallFunction|ClearSwitchAreaInfo _output_get))
    (:else)))

(fn TogglePrimaryAbility
  (params (pressed/Released :type Boolean) (playerRef :type BP%20Main%20Character%20Object%20Reference))
  (bind _switchableactors (Variables|Default|GetswitchableActors))
  (|CallParentFunction pressed/Released playerRef)
  (if pressed/Released
    (if (Utilities|Array|IsNotEmpty _switchableactors)
      (CallFunction|SwitchState _switchableactors (Variables|Default|GetglobalState)))))

(fn ToggleSecundaryAbility
  (params (pressed/Released :type Boolean) (playerRef :type BP%20Main%20Character%20Object%20Reference))
  (|CallParentFunction pressed/Released playerRef))

(fn ResetHighPriestress
  (CallFunction|ToggleSwitchState false)
  (Variables|Default|Setin%20changing%20state false))

(fn FindSwitchArea
  (Variables|Default|SetcurrSwitchArea 0)
  (bind _outactors (Collision|SphereOverlapActors (Transformation|GetActorLocation (Game|GetPlayerCharacter 0)) 2e+01 (Utilities|Array|MakeArray "ObjectTypeQuery2") "/Game/Arxcana/Core/SwitchableObjects/BP_SwitchArea.BP_SwitchArea_C"))
  (if (Utilities|Array|IsNotEmpty _outactors)
    (bind _asbp_switch_area (Utilities|Casting|CastToBP_SwitchArea (Utilities|Array|Get(acopy) _outactors)))
    (Variables|Default|SetcurrSwitchArea _asbp_switch_area)
    (Variables|Default|SetglobalState (Variables|/Game/Arxcana/Core/SwitchableObjects/BP_SwitchArea.BP_SwitchArea_C|GetareaState _asbp_switch_area))
    (bind _switchableobjects (Default|GetSwitchableObjects _asbp_switch_area))
    (Variables|Default|SetswitchableActors _switchableobjects)
    (return true)
    (else
      (return false))))

(fn ClearSwitchAreaInfo
  (params (lastState :type BPE_HighPriestressState%20Enum :default "NewEnumerator0"))
  (Utilities|Array|Clear (Variables|Default|GetswitchableActors))
  (Variables|Default|SetglobalState lastState))

(fn SwitchState
  (params (affectedActors :type Array%20of%20Actor%20Object%20References) (stateToSwitchOn :type BPE_HighPriestressState%20Enum :default "NewEnumerator0"))
  (switch Utilities|FlowControl|Switch|SwitchonBPE_HighPriestressState stateToSwitchOn
    (:NewEnumerator0
      (bind _output_get (Variables|Default|SetglobalState "NewEnumerator1"))
      (Development|PrintString "Switched to state B")
      (for _array_element (Variables|Default|GetswitchableActors)
        (Class|BPISwitchable|SwitchState(Message) _array_element _output_get)))
    (:NewEnumerator1
      (bind _output_get_2 (Variables|Default|SetglobalState "NewEnumerator0"))
      (Development|PrintString "Switched to state A")
      (for _array_element_2 (Variables|Default|GetswitchableActors)
        (Class|BPISwitchable|SwitchState(Message) _array_element_2 _output_get_2)))))

(fn ToggleSwitchState
  (params (enter/Exit :type Boolean))
  (bind _globalstate (Variables|Default|GetglobalState))
  (if (Utilities|Array|IsNotEmpty (Variables|Default|GetswitchableActors))
    (if enter/Exit
      (for _array_element (Variables|Default|GetswitchableActors)
        (bind _asbp_switchable_object (Utilities|Casting|CastToBP_SwitchableObject _array_element))
        (Default|EnterChangingState _asbp_switchable_object _globalstate "/Game/Arxcana/MaterialLibrary/HighPriestess_Fog/MM_HighPriestess_Fog.MM_HighPriestess_Fog"))
      (else
        (for _array_element_2 (Variables|Default|GetswitchableActors)
          (bind _asbp_switchable_object_2 (Utilities|Casting|CastToBP_SwitchableObject _array_element_2))
          (Default|ExitChangingState _asbp_switchable_object_2 _globalstate))))
    (else
      (Development|PrintString "There are no switchable actors!"))))

(fn AssignSwitchAreaInfo
  (params (switchableActors :type Array%20of%20Actor%20Object%20References) (globalState :type BPE_HighPriestressState%20Enum :default "NewEnumerator0"))
  (Variables|Default|SetswitchableActors switchableActors)
  (Variables|Default|SetglobalState globalState))