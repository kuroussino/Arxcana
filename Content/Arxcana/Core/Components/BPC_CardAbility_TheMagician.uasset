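; The Magician card ability component, which lets the player grab and carry BPI_Grabbable objects from a distance.
; Pressing the primary ability line-traces from the camera and attaches the hit to the character's PhysicsHandle; releasing drops it.
; Tick holds the object at its initial distance along the view with spin zeroed, dropping it if the trace misses while it moves too fast.
; When idle, delayed traces drive LookAt and StopLookAt feedback.
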(event EventTick
  (params (DeltaSeconds :type Float%20%28single-precision%29))
  (bind _returnvalue (Game|GetPlayerCameraManager 0))
  (bind _rootcomponent (Variables|/Script/Engine.Actor|GetRootComponent _returnvalue))
  (if (Variables|Default|GetisGrabbingObject)
    (Utilities|TryGrab (Variables|/Script/Engine.Actor|GetRootComponent (Game|GetPlayerCameraManager 0)) (Variables|Default|GetgrabDistance)
      (:true
        (bind _asbp_main_character (Utilities|Casting|CastToBP_MainCharacter (Game|GetPlayerCharacter 0) :!label _label))
        (Physics|Components|PhysicsHandle|SetTargetLocation (Variables|/Game/Arxcana/Core/MainCharacter/BP_MainCharacter.BP_MainCharacter_C|GetPhysicsHandle _asbp_main_character) (+ (Transformation|GetWorldLocation _rootcomponent) (* (Math|Vector|GetForwardVector (Transformation|GetWorldRotation _rootcomponent)) (Variables|Default|GetcurrGrabbedObjDistance))))
        (bind _staticmesh (Default|GetStaticMesh (Variables|Default|GetcurrGrabbedObjInterfaceRef)))
        (Class|PrimitiveComponent|SetPhysicsAngularVelocityinDegrees _staticmesh "0, 0, 0" false "None"))
      (:false
        (Development|PrintString (Utilities|String|Append "current velocity: " (Utilities|String|ToString(Float) (Math|Vector|VectorLength (Transformation|GetComponentVelocity (Class|PhysicsHandleComponent|GetGrabbedComponent (Variables|/Game/Arxcana/Core/MainCharacter/BP_MainCharacter.BP_MainCharacter_C|GetPhysicsHandle _asbp_main_character)))))))
        (if (> (Math|Vector|VectorLength (Transformation|GetComponentVelocity (Class|PhysicsHandleComponent|GetGrabbedComponent (Variables|/Game/Arxcana/Core/MainCharacter/BP_MainCharacter.BP_MainCharacter_C|GetPhysicsHandle _asbp_main_character)))) (Variables|Default|GetvelocityTreshold))
          (CallFunction|EndGrab)
          (else
            (goto _label)))))
    (else
      (Utilities|FlowControl|Delay 0.1)
      (bind (_as_bpi_grabbable _hitactor) (Utilities|TryGrab (Variables|/Script/Engine.Actor|GetRootComponent (Game|GetPlayerCameraManager 0)) (Variables|Default|GetgrabDistance))
        (:true
          (Default|Lookat _as_bpi_grabbable)
          (bind _lookatactor (Variables|Default|GetlookAtActor)
            (:then
              (if (== _lookatactor _hitactor)
                _
                (else
                  (bind _asbpi_grabbable (Utilities|Casting|CastToBPI_Grabbable _lookatactor))
                  (Default|StopLookat _asbpi_grabbable))))
            (:else
              _))
          (Variables|Default|SetlookAtActor _hitactor))
        (:false
          (bind _asbpi_grabbable_2 (Utilities|Casting|CastToBPI_Grabbable (Variables|Default|GetlookAtActor)))
          (Default|StopLookat _asbpi_grabbable_2))))))

(fn TogglePrimaryAbility
  (params (pressed/Released :type Boolean) (playerRef :type BP%20Main%20Character%20Object%20Reference))
  (|CallParentFunction pressed/Released playerRef)
  (if pressed/Released
    (bind (_as_bpi_grabbable _hitactor _hitcomponent) (Utilities|TryGrab (Variables|/Script/Engine.Actor|GetRootComponent (Game|GetPlayerCameraManager 0)) (Variables|Default|GetgrabDistance))
      (:true
        (Variables|Default|SetisGrabbingObject true)
        (Development|PrintString "Begin Grab")
        (Class|PhysicsHandleComponent|GrabComponentatLocation (Variables|/Game/Arxcana/Core/MainCharacter/BP_MainCharacter.BP_MainCharacter_C|GetPhysicsHandle playerRef) _hitcomponent "None" (Transformation|GetWorldLocation _hitcomponent))
        (Variables|Default|SetcurrGrabbedObj _hitactor)
        (Variables|Default|SetcurrGrabbedObjInterfaceRef _as_bpi_grabbable)
        (Variables|Default|SetcurrGrabbedObjDistance (Math|Vector|Distance(Vector) (Transformation|GetWorldLocation _hitcomponent) (Transformation|GetWorldLocation (Variables|/Script/Engine.Actor|GetRootComponent (Game|GetPlayerCameraManager 0)))))))
    (else
      (CallFunction|EndGrab))))

(fn EndGrab
  (if (Variables|Default|GetisGrabbingObject)
    (Variables|Default|SetisGrabbingObject false)
    (Development|PrintString "End Grab")
    (bind _asbp_main_character (Utilities|Casting|CastToBP_MainCharacter (Game|GetPlayerCharacter 0)))
    (Physics|Components|PhysicsHandle|ReleaseComponent (Variables|/Game/Arxcana/Core/MainCharacter/BP_MainCharacter.BP_MainCharacter_C|GetPhysicsHandle _asbp_main_character))
    (Variables|Default|SetcurrGrabbedObj 0)
    (Variables|Default|SetcurrGrabbedObjDistance 0.0)
    (Variables|Default|SetcurrGrabbedObjInterfaceRef 0)))