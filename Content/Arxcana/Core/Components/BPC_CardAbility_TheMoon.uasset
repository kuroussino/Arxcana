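; Card ability component for The Moon tarot card, driving its press-and-hold primary ability.
; TogglePrimaryAbility extends the parent version, then casts the player's held card to BP_Card_TheMoon and forwards the pressed state through ToggleFunction.
; Pressing stops the player's levitation animation, while releasing re-enables levitation and restarts that animation.
; The effect itself lives in the card actor, and the event graph is empty.
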(event EventBeginPlay)

(event EventTick
  (params (DeltaSeconds :type Float%20%28single-precision%29)))

(fn TogglePrimaryAbility
  (params (pressed/Released :type Boolean) (playerRef :type BP%20Main%20Character%20Object%20Reference))
  (|CallParentFunction pressed/Released playerRef)
  (if pressed/Released
    (Default|StopLevitationAnimation playerRef)
    (bind _asbp_card_the_moon (Utilities|Casting|CastToBP_Card_TheMoon (Variables|/Game/Arxcana/Core/MainCharacter/BP_MainCharacter.BP_MainCharacter_C|GetcardInHand playerRef)))
    (Default|ToggleFunction _asbp_card_the_moon true)
    (else
      (Variables|/Game/Arxcana/Core/MainCharacter/BP_MainCharacter.BP_MainCharacter_C|SetcanLevitate playerRef true)
      (Default|StartLevitaionAnimation playerRef)
      (bind _asbp_card_the_moon_2 (Utilities|Casting|CastToBP_Card_TheMoon (Variables|/Game/Arxcana/Core/MainCharacter/BP_MainCharacter.BP_MainCharacter_C|GetcardInHand playerRef)))
      (Default|ToggleFunction _asbp_card_the_moon_2 false))))