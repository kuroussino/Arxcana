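; Card carousel actor that displays the player's owned cards in a ring for browsing and choosing one.
; SpawnCards reorders the cards to start at the last index, then spawns them evenly around a rotating scene component using a stepped arrow.
; Selection changes spin the ring and scale cards through timelines, then update the character's tips.
; ChooseCard returns the selected class; destruction saves index and order to BP_MainCharacter and destroys the spawned cards.
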(event Custom|SpawnCards
  (params (lastIndex :type Integer) (cardsownedRef :type Array%20of%20Actor%20Class%20References))
  (bind _currentspawnorder (Variables|Default|GetcurrentSpawnOrder))
  ;[0.4118 0 1] Pre-Spawn Check
  (Variables|Default|Setrotating true)
  (Variables|Default|SetcurrentCardIndex 0)
  (bind _asbp_main_character (Utilities|Casting|CastToBP_MainCharacter (Game|GetPlayerCharacter 0)))
  (if (> (Utilities|Array|Length (Variables|/Game/Arxcana/Core/MainCharacter/BP_MainCharacter.BP_MainCharacter_C|GetcardsOwned _asbp_main_character)) (Utilities|Array|Length cardsownedRef))
    (bind _output_get (Variables|Default|SetcardsOwnedRef (Variables|/Game/Arxcana/Core/MainCharacter/BP_MainCharacter.BP_MainCharacter_C|GetcardsOwned _asbp_main_character)))
    (if (> (Utilities|Array|Length _output_get) 0)
      (CallFunction|CheckRotationOffset :!label _label)
      (Utilities|FlowControl|Delay 0.1)
      ;[0.4118 0 1] Sort Cards
      (for _index (range lastIndex (- (Utilities|Array|Length (Variables|Default|GetcardsOwnedRef)) 1))
        (Utilities|Array|AddUnique (Variables|Default|GetcurrentSpawnOrder) (Utilities|Array|Get(acopy) (Variables|Default|GetcardsOwnedRef) _index)))
      (for _index_2 (range 0 (- lastIndex 1))
        (Utilities|Array|AddUnique (Variables|Default|GetcurrentSpawnOrder) (Utilities|Array|Get(acopy) (Variables|Default|GetcardsOwnedRef) _index_2)))
      (Variables|Default|SetcardsOwnedRef _currentspawnorder)
      ;[0.4118 0 1] Spawn Cards
      (for _array_element _currentspawnorder
        (Development|PrintString (Utilities|GetClassDisplayName _array_element))
        (bind _newspawnlocation (CallFunction|GetCardSpawnLocation true))
        (bind _returnvalue (Game|SpawnActorfromClass _array_element (Math|Transform|MakeTransform _newspawnlocation "0, 0, 0" "1.000000,1.000000,1.000000") "AlwaysSpawn" "MultiplyWithRoot" 0 0))
        (Utilities|Array|AddUnique (Variables|Default|GetspawnedCards) _returnvalue)
        (Transformation|AttachComponentToComponent _returnvalue (Variables|Default|GetScene) "None" "KeepWorld" "KeepWorld" "KeepWorld" true)
        (Transformation|SetActorRelativeRotation _returnvalue)
        (Variables|Default|Setrotating false))
      (CallFunction|ResetSpawnArrow)
      (CallFunction|ScaleUpCard)
      (else
        (Development|PrintString "You don't have any card" :!label _label_2)))
    (else
      (bind _output_get_2 (Variables|Default|SetcardsOwnedRef cardsownedRef))
      (if (> (Utilities|Array|Length _output_get_2) 0)
        (goto _label)
        (else
          (goto _label_2))))))

(event Custom|RotateCarousel
  (params (Right/Left :type Boolean))
  ;[0 1 0.05882] Rotate Carousel
  (Variables|Default|Setrotating true)
  (if Right/Left
    (Components|Timeline|SetPlayRate (Variables|Default|GetTimeline) (/ 1.0 (Variables|Default|GetrotationDuration)))
    (Variables|Default|SetcurrTargetZ (.yaw (Variables|/Script/Engine.SceneComponent|GetRelativeRotation (Variables|Default|GetScene))))
    (Variables|Default|SetcurrStartRot (Transformation|GetActorRotation))
    (bind _0_1 (Timeline|Timeline PlayFromStart)
      (:Update
        (Transformation|SetRelativeRotation (Variables|Default|GetScene) (Math|Rotator|MakeRotator 0.0 0.0 (+ (Variables|Default|GetcurrTargetZ) (* _0_1 (Variables|Default|GetrotationOffset)))) false false))
      (:Finished
        (CallFunction|ScaleUpCard)
        (Development|PrintString (Utilities|String|ToString(Integer) (Variables|Default|GetcurrentCardIndex)))))
    (else
      (Components|Timeline|SetPlayRate (Variables|Default|GetTimeline_1) (/ 1.0 (Variables|Default|GetrotationDuration)))
      (Variables|Default|SetcurrTargetZ (.yaw (Variables|/Script/Engine.SceneComponent|GetRelativeRotation (Variables|Default|GetScene))))
      (Variables|Default|SetcurrStartRot (Transformation|GetActorRotation))
      (bind _0_1_2 (Timeline|Timeline_1 PlayFromStart)
        (:Update
          (Transformation|SetRelativeRotation (Variables|Default|GetScene) (Math|Rotator|MakeRotator 0.0 0.0 (- (Variables|Default|GetcurrTargetZ) (* _0_1_2 (Variables|Default|GetrotationOffset)))) false false))
        (:Finished
          (CallFunction|ScaleUpCard)
          (Development|PrintString (Utilities|String|ToString(Integer) (Variables|Default|GetcurrentCardIndex))))))))

(event Custom|ScaleDownCard
  (params (index :type Integer))
  ;[0 1 0.05882] Scale Selected Card
  (Components|Timeline|SetPlayRate (Variables|Default|GetTimeline_2) (/ 1.0 0.3))
  (bind _1_25_1 (Timeline|Timeline_2 PlayFromStart)
    (:Update
      (Transformation|SetActorRelativeScale3D (Utilities|Array|Get(acopy) (Variables|Default|GetspawnedCards) index) (Math|Conversions|ToVector(Float) _1_25_1)))))

(event Custom|ScaleUpCard
  (params (index :type Integer))
  ;[0 1 0.05882] Scale Selected Card
  (Variables|Default|Setrotating true)
  (Components|Timeline|SetPlayRate (Variables|Default|GetTimeline_0) (/ 1.0 0.3))
  (bind _1_1_25 (Timeline|Timeline_0 PlayFromStart)
    (:Update
      (Transformation|SetActorRelativeScale3D (Utilities|Array|Get(acopy) (Variables|Default|GetspawnedCards) (Variables|Default|GetcurrentCardIndex)) (Math|Conversions|ToVector(Float) _1_1_25)))
    (:Finished
      (Variables|Default|Setrotating false))))

(event EventTick
  (params (DeltaSeconds :type Float%20%28single-precision%29))
  ;[0.6627 0 0] Update Z Rot
  (Transformation|SetActorRotation (Math|Rotator|MakeRotator 0.0 0.0 (.yaw (Transformation|GetActorRotation)))))

(event EventDestroyed
  ;[0.6627 0 0] OnDestroyed
  (bind _asbp_main_character (Utilities|Casting|CastToBP_MainCharacter (Game|GetPlayerCharacter 0)))
  (Default|SaveLastCarouselIndex _asbp_main_character (Variables|Default|GetcurrentCardIndex) (Variables|Default|GetcardsOwnedRef))
  (for _array_element (Variables|Default|GetspawnedCards)
    (Actor|DestroyActor _array_element)))

(fn ConstructionScript)

(fn CheckRotationOffset
  (Variables|Default|SetrotationOffset (Math|Conversions|ToFloat(Integer) (/ 360 (Utilities|Array|Length (Variables|Default|GetcardsOwnedRef))))))

(fn GetCardSpawnLocation
  (params (rotateByOffset%20%28after%29 :type Boolean))
  (bind _arrow (Variables|Default|GetArrow))
  (if rotateByOffset%20%28after%29
    (bind _output_get (Variables|Default|SetcurrentSpawnLocation (+ (Transformation|GetWorldLocation _arrow) (* (Math|Vector|Normalize (Math|Vector|GetForwardVector _arrow)) (Variables|Default|GetspawnRadius)))))
    (Transformation|AddLocalRotation (Variables|Default|GetArrow) (Math|Rotator|MakeRotator 0.0 0.0 (Variables|Default|GetrotationOffset)) false false))
  (return _output_get))

(fn ResetSpawnArrow
  (Transformation|SetRelativeRotation (Variables|Default|GetArrow) "0, 0, 0" false false))

(fn SelectFollowing/PreviousCard
  (params (Following/Previous :type Boolean))
  (if (> (Utilities|Array|Length (Variables|Default|GetspawnedCards)) 1)
    (if Following/Previous
      (CallFunction|RotateCarousel false)
      (CallFunction|ScaleDownCard (Variables|Default|GetcurrentCardIndex))
      (if (> (+ (Variables|Default|GetcurrentCardIndex) 1) (- (Utilities|Array|Length (Variables|Default|GetcardsOwnedRef)) 1))
        (Variables|Default|SetcurrentCardIndex 0)
        (else
          (Math|Integer|IncrementInt (Variables|Default|GetcurrentCardIndex)
            (:%20%20
              _))))
      (else
        (CallFunction|RotateCarousel true)
        (CallFunction|ScaleDownCard (Variables|Default|GetcurrentCardIndex))
        (if (< (- (Variables|Default|GetcurrentCardIndex) 1) 0)
          (Variables|Default|SetcurrentCardIndex (- (Utilities|Array|Length (Variables|Default|GetcardsOwnedRef)) 1))
          (else
            (Math|Integer|DecrementInt (Variables|Default|GetcurrentCardIndex)
              (:%20%20
                _))))))
    (bind _asbp_main_character (Utilities|Casting|CastToBP_MainCharacter (Game|GetPlayerCharacter 0)))
    (Default|GetCurrentSelectedCardandUpdateTips _asbp_main_character)))

(fn ChooseCard
  (if (> (Utilities|Array|Length (Variables|Default|GetcardsOwnedRef)) 0)
    (return (Utilities|Array|Get(acopy) (Variables|Default|GetcurrentSpawnOrder) (Variables|Default|GetcurrentCardIndex)) true)
    (else
      (return 0 false))))