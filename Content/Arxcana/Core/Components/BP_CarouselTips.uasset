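; BP_CarouselTips is an actor that shows tip text, judging by its name for a carousel, and keeps itself facing the player's camera.
; On BeginPlay it snaps its yaw toward the camera, then each Tick smoothly interpolates pitch and yaw to follow the camera like a billboard.
; A ChangeText function sets the string on its TextRender component.
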(event EventBeginPlay
  (Transformation|SetActorRotation (Math|Rotator|MakeRotator 0.0 0.0 (.yaw (Math|Rotator|FindLookatRotation (Transformation|GetActorLocation) (Camera|GetCameraLocation (Game|GetPlayerCameraManager 0)))))))

(event Collision|EventActorBeginOverlap
  (params (OtherActor :type Actor%20Object%20Reference)))

(event EventTick
  (params (DeltaSeconds :type Float%20%28single-precision%29))
  (bind _returnvalue (Transformation|GetActorLocation))
  (bind _returnvalue_2 (Game|GetPlayerCameraManager 0))
  (bind _returnvalue_3 (Transformation|GetActorRotation))
  (bind _returnvalue_4 (Camera|GetCameraLocation _returnvalue_2))
  (bind _returnvalue_5 (Math|Rotator|FindLookatRotation _returnvalue _returnvalue_4))
  (bind _returnvalue_6 (Math|Interpolation|RInterpTo _returnvalue_3 _returnvalue_5 DeltaSeconds 5.0))
  (Transformation|SetActorRotation (Math|Rotator|MakeRotator 0.0 (.pitch _returnvalue_6) (.yaw _returnvalue_6))))

(fn ConstructionScript)

(fn ChangeText
  (params (text :type Text))
  (Rendering|Components|TextRender|SetText (Variables|Default|GetTextRender) text))