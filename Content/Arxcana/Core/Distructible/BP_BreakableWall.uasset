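; BP_BreakableWall is a wall actor that starts hidden and inert, then is destroyed after player contact once enabled.
; BeginPlay calls Disable, which hides it and turns off its collision and physics.
; Enable, not called within this Blueprint, reverses this and sets HasSpawned.
; With that flag set, the player character overlapping BreakCheck triggers destruction after a short delay.
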(event OnComponentBeginOverlap(BreakCheck)
  (params (OverlappedComponent :type Primitive%20Component%20Object%20Reference) (OtherActor :type Actor%20Object%20Reference) (OtherComp :type Primitive%20Component%20Object%20Reference) (OtherBodyIndex :type Integer) (bFromSweep :type Boolean) (SweepResult :type Hit%20Result%20Structure%20%28by%20ref%29))
  (if (Variables|Default|GethasSpawned)
    (if (== OtherActor (Game|GetPlayerCharacter 0))
      (Utilities|FlowControl|Delay 2.0)
      (Actor|DestroyActor))))

(event EventBeginPlay
  (CallFunction|Disable)
  (Variables|Default|SethasSpawned false))

(event Collision|EventActorBeginOverlap
  (params (OtherActor :type Actor%20Object%20Reference)))

(event EventTick
  (params (DeltaSeconds :type Float%20%28single-precision%29)))

(fn ConstructionScript)

(fn Disable
  (Development|PrintString "Wall disabled")
  (Physics|SetSimulatePhysics (Variables|Default|GetBreakableWall) false)
  (Collision|SetCollisionEnabled (Variables|Default|GetBreakableWall) "NoCollision")
  (Rendering|SetActorHiddenInGame true))

(fn Enable
  (bind _breakablewall (Variables|Default|GetBreakableWall))
  (Development|PrintString "Wall enabled")
  (Collision|SetCollisionEnabled _breakablewall "QueryAndPhysics")
  (Rendering|SetActorHiddenInGame false)
  (Physics|SetSimulatePhysics _breakablewall true)
  (Variables|Default|SethasSpawned true))