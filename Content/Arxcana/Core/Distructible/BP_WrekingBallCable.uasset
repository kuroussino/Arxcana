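; Wrecking ball cable actor that hooks up a BP_WrekingBallSphere when it enters the Box trigger.
; On overlap it makes the player's BP_MainCharacter release its grabbed object, then attaches the sphere actor to itself, keeping world transforms.
; The sphere's mesh is then physics-constrained to Base, set as the Cable component's end, and given a higher mass scale.
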(event OnComponentBeginOverlap(Box)
  (params (OverlappedComponent :type Primitive%20Component%20Object%20Reference) (OtherActor :type Actor%20Object%20Reference) (OtherComp :type Primitive%20Component%20Object%20Reference) (OtherBodyIndex :type Integer) (bFromSweep :type Boolean) (SweepResult :type Hit%20Result%20Structure%20%28by%20ref%29))
  (if (== (Utilities|GetClass OtherActor) "/Game/Arxcana/Core/Distructible/BP_WrekingBallSphere.BP_WrekingBallSphere_C")
    (bind _asbp_main_character (Utilities|Casting|CastToBP_MainCharacter (Game|GetPlayerCharacter 0)))
    (Default|UnGrabObject _asbp_main_character)
    (Transformation|AttachActorToActor OtherActor self "None" "KeepWorld" "KeepWorld" "KeepWorld" true)
    (bind _staticmesh (Class|BPIGrabbable|GetStaticMesh(Message) OtherActor))
    (Class|PhysicsConstraintComponent|SetConstrainedComponents (Variables|Default|GetPhysicsConstraint) (Variables|Default|GetBase) "None" _staticmesh "None")
    (Class|CableComponent|SetAttachEndtoComponent (Variables|Default|GetCable) _staticmesh "None")
    (Class|PrimitiveComponent|SetMassScale _staticmesh "None" 5.0)))

(fn ConstructionScript)