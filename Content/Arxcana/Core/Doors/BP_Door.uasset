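; BP_Door is a two-leaf sliding door that opens for the player character and slides back when the player leaves.
; Each leaf has its own detection component and timeline, played on begin overlap and reversed on end overlap.
; The timelines lerp relative location from zero toward DoorDXSlideDistance for DoorSx and its negation for DoorDx.
; The Closed flag blocks both the opening and reversing triggers.
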(event OnComponentBeginOverlap(DoorDetectionSX)
  (params (OverlappedComponent :type Primitive%20Component%20Object%20Reference) (OtherActor :type Actor%20Object%20Reference) (OtherComp :type Primitive%20Component%20Object%20Reference) (OtherBodyIndex :type Integer) (bFromSweep :type Boolean) (SweepResult :type Hit%20Result%20Structure%20%28by%20ref%29))
  ;[0 0.1432 1] DoorSliding
  (if (and (== OtherActor (Game|GetPlayerCharacter 0)) (not (Variables|Default|Getclosed)))
    (bind _doorslidef (Timeline|Door%20Opening Play)
      (:Update
        (Transformation|SetRelativeLocation (Variables|Default|GetDoorSx) (Math|Vector|Lerp(Vector) "0, 0, 0" (Variables|Default|GetDoorDXSlideDistance) _doorslidef) false false)))))

(event OnComponentBeginOverlap(DoorDetectionDx)
  (params (OverlappedComponent :type Primitive%20Component%20Object%20Reference) (OtherActor :type Actor%20Object%20Reference) (OtherComp :type Primitive%20Component%20Object%20Reference) (OtherBodyIndex :type Integer) (bFromSweep :type Boolean) (SweepResult :type Hit%20Result%20Structure%20%28by%20ref%29))
  ;[0 0.1432 1] DoorSliding
  (if (and (== OtherActor (Game|GetPlayerCharacter 0)) (not (Variables|Default|Getclosed)))
    (bind _doorslidef (Timeline|Timeline Play)
      (:Update
        (Transformation|SetRelativeLocation (Variables|Default|GetDoorDx) (Math|Vector|Lerp(Vector) "0, 0, 0" (* (Variables|Default|GetDoorDXSlideDistance) -1.0) _doorslidef) false false)))))

(event OnComponentEndOverlap(DoorDetectionDx)
  (params (OverlappedComponent :type Primitive%20Component%20Object%20Reference) (OtherActor :type Actor%20Object%20Reference) (OtherComp :type Primitive%20Component%20Object%20Reference) (OtherBodyIndex :type Integer))
  ;[0 0.1432 1] DoorSliding
  (if (and (== OtherActor (Game|GetPlayerCharacter 0)) (not (Variables|Default|Getclosed)))
    (bind _doorslidef (Timeline|Timeline Reverse)
      (:Update
        (Transformation|SetRelativeLocation (Variables|Default|GetDoorDx) (Math|Vector|Lerp(Vector) "0, 0, 0" (* (Variables|Default|GetDoorDXSlideDistance) -1.0) _doorslidef) false false)))))

(event OnComponentEndOverlap(DoorDetectionSX)
  (params (OverlappedComponent :type Primitive%20Component%20Object%20Reference) (OtherActor :type Actor%20Object%20Reference) (OtherComp :type Primitive%20Component%20Object%20Reference) (OtherBodyIndex :type Integer))
  ;[0 0.1432 1] DoorSliding
  (if (and (== OtherActor (Game|GetPlayerCharacter 0)) (not (Variables|Default|Getclosed)))
    (bind _doorslidef (Timeline|Door%20Opening Reverse)
      (:Update
        (Transformation|SetRelativeLocation (Variables|Default|GetDoorSx) (Math|Vector|Lerp(Vector) "0, 0, 0" (Variables|Default|GetDoorDXSlideDistance) _doorslidef) false false)))))

(event EventBeginPlay)

(event Collision|EventActorBeginOverlap
  (params (OtherActor :type Actor%20Object%20Reference)))

(event EventTick
  (params (DeltaSeconds :type Float%20%28single-precision%29)))

(fn ConstructionScript)