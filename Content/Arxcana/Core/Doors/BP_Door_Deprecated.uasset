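; Deprecated torch-puzzle double sliding door that leads to the next level.
; Torch active-check events re-evaluate the puzzle, opening the door when all listed torches have the required point-light visibility.
; Two timelines slide the leaves in opposite directions, replayed or reversed by per-side player overlaps while unlocked.
; After a puzzle solve, entering the SX trigger instead warps the player once through the main character's WarpManager.
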(event OnComponentBeginOverlap(DoorDetectionSX)
  (params (OverlappedComponent :type Primitive%20Component%20Object%20Reference) (OtherActor :type Actor%20Object%20Reference) (OtherComp :type Primitive%20Component%20Object%20Reference) (OtherBodyIndex :type Integer) (bFromSweep :type Boolean) (SweepResult :type Hit%20Result%20Structure%20%28by%20ref%29))
  (bind _returnvalue (Game|GetPlayerCharacter 0))
  ;[0 0.1432 1] DoorSliding
  (if (== OtherActor _returnvalue)
    (if (Variables|Default|GetneedsToWarp)
      (Utilities|FlowControl|DoOnce false
        (:Completed
          (bind _asbp_main_character (Utilities|Casting|CastToBP_MainCharacter _returnvalue))
          (Default|WarptoNextLevel (Variables|/Game/Arxcana/Core/MainCharacter/BP_MainCharacter.BP_MainCharacter_C|GetwarpManager _asbp_main_character))))
      (elif (and (== OtherActor _returnvalue) (not (Variables|Default|Getclosed)))
        (bind _doorslidef (Timeline|Door%20Opening Play)
          (:Update
            (Transformation|SetRelativeLocation (Variables|Default|GetDoorSx) (Math|Vector|Lerp(Vector) "0, 0, 0" (Variables|Default|GetDoorDXSlideDistance) _doorslidef) false false)))))))

(event OnComponentBeginOverlap(DoorDetectionDx)
  (params (OverlappedComponent :type Primitive%20Component%20Object%20Reference) (OtherActor :type Actor%20Object%20Reference) (OtherComp :type Primitive%20Component%20Object%20Reference) (OtherBodyIndex :type Integer) (bFromSweep :type Boolean) (SweepResult :type Hit%20Result%20Structure%20%28by%20ref%29))
  ;[0 0.1432 1] DoorSliding
  (if (and (== OtherActor (Game|GetPlayerCharacter 0)) (not (Variables|Default|Getclosed)))
    (bind _doorslidef (Timeline|Timeline Play)
      (:Update
        (Transformation|SetRelativeLocation (Variables|Default|GetDoorDx) (Math|Vector|Lerp(Vector) "0, 0, 0" (* (Variables|Default|GetDoorDXSlideDistance) -1.0) _doorslidef) false false)))))

(event OnComponentEndOverlap(DoorDetectionDx)
  (params (OverlappedComponent :type Primitive%20Component%20Object%20Reference) (OtherActor :type Actor%20Object%20Reference) (OtherComp :type Primitive%20Component%20Object%20Reference) (OtherBodyIndex :type Integer))
  ;[0 0.1432 1] DoorSliding
  (if (Variables|Default|GetautomaticClose)
    (if (and (== OtherActor (Game|GetPlayerCharacter 0)) (not (Variables|Default|Getclosed)))
      (bind _doorslidef (Timeline|Timeline Reverse)
        (:Update
          (Transformation|SetRelativeLocation (Variables|Default|GetDoorDx) (Math|Vector|Lerp(Vector) "0, 0, 0" (* (Variables|Default|GetDoorDXSlideDistance) -1.0) _doorslidef) false false))))))

(event OnComponentEndOverlap(DoorDetectionSX)
  (params (OverlappedComponent :type Primitive%20Component%20Object%20Reference) (OtherActor :type Actor%20Object%20Reference) (OtherComp :type Primitive%20Component%20Object%20Reference) (OtherBodyIndex :type Integer))
  ;[0 0.1432 1] DoorSliding
  (if (Variables|Default|GetautomaticClose)
    (if (and (== OtherActor (Game|GetPlayerCharacter 0)) (not (Variables|Default|Getclosed)))
      (bind _doorslidef (Timeline|Door%20Opening Reverse)
        (:Update
          (Transformation|SetRelativeLocation (Variables|Default|GetDoorSx) (Math|Vector|Lerp(Vector) "0, 0, 0" (Variables|Default|GetDoorDXSlideDistance) _doorslidef) false false))))))

(event Custom|CloseDoor
  (bind _doordxslidedistance (Variables|Default|GetDoorDXSlideDistance))
  (Variables|Default|SetautomaticClose false)
  (Variables|Default|Setclosed true)
  (Utilities|FlowControl|Sequence
    (:then_0
      ;[0 0.1432 1] DoorSliding
      (bind _doorslidef (Timeline|Door%20Opening Reverse)
        (:Update
          (Transformation|SetRelativeLocation (Variables|Default|GetDoorSx) (Math|Vector|Lerp(Vector) "0, 0, 0" _doordxslidedistance _doorslidef) false false))))
    (:then_1
      (bind _doorslidef_2 (Timeline|Timeline Reverse)
        (:Update
          (Transformation|SetRelativeLocation (Variables|Default|GetDoorDx) (Math|Vector|Lerp(Vector) "0, 0, 0" (* _doordxslidedistance -1.0) _doorslidef_2) false false))))))

(event Custom|CheckToches
  (if (Variables|Default|Getclosed)
    (bind _allactive (CallFunction|CheckTorches))
    (if _allactive
      (CallFunction|OpenDoor)
      (Development|PrintString "Door opened!")
      (Variables|Default|SetneedsToWarp true))))

(event Custom|OpenDoor
  (bind _doordxslidedistance (Variables|Default|GetDoorDXSlideDistance))
  (Variables|Default|SetautomaticClose true)
  (Variables|Default|Setclosed false)
  (Utilities|FlowControl|Sequence
    (:then_0
      ;[0 0.1432 1] DoorSliding
      (bind _doorslidef (Timeline|Timeline PlayFromStart)
        (:Update
          (Transformation|SetRelativeLocation (Variables|Default|GetDoorDx) (Math|Vector|Lerp(Vector) "0, 0, 0" (* _doordxslidedistance -1.0) _doorslidef) false false))))
    (:then_1
      (bind _doorslidef_2 (Timeline|Door%20Opening PlayFromStart)
        (:Update
          (Transformation|SetRelativeLocation (Variables|Default|GetDoorSx) (Math|Vector|Lerp(Vector) "0, 0, 0" _doordxslidedistance _doorslidef_2) false false))))))

(event EventBeginPlay
  (if (or (Utilities|Array|IsNotEmpty (Variables|Default|GettorchesToEnable)) (Utilities|Array|IsNotEmpty (Variables|Default|GettorchesToDisable)))
    (for _array_element (Variables|Default|GettorchesToEnable)
      (EventDispatchers|BindEventtoActiveCheck _array_element (delegate Custom|CheckToches)))
    (for _array_element_2 (Variables|Default|GettorchesToDisable)
      (EventDispatchers|BindEventtoActiveCheck _array_element_2 (delegate Custom|CheckToches)))))

(fn ConstructionScript)

(fn CheckTorches
  (Variables|Default|SetactiveTorches 0)
  (Variables|Default|SetdisabledTorches 0)
  (for _array_element (Variables|Default|GettorchesToEnable)
    (if (Rendering|IsVisible (Variables|/Game/Arxcana/Core/LaserSystem/BP_IgnitableTorch.BP_IgnitableTorch_C|GetPointLight _array_element))
      (Math|Integer|IncrementInt (Variables|Default|GetactiveTorches))))
  (for _array_element_2 (Variables|Default|GettorchesToDisable)
    (if (not (Rendering|IsVisible (Variables|/Game/Arxcana/Core/LaserSystem/BP_IgnitableTorch.BP_IgnitableTorch_C|GetPointLight _array_element_2)))
      (Math|Integer|IncrementInt (Variables|Default|GetdisabledTorches))))
  (if (and (== (Variables|Default|GetactiveTorches) (Utilities|Array|Length (Variables|Default|GettorchesToEnable))) (== (Variables|Default|GetdisabledTorches) (Utilities|Array|Length (Variables|Default|GettorchesToDisable))))
    (return true)
    (else
      (return false))))