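; Moving platform that buttons enable and disable, travelling between its start location and target points converted to world space at BeginPlay.
; A timeline lerps the platform over the cycle duration, with Ping Pong behaviour reversing it through a direction flag.
; It either waits for a required button count or, with SwitchLocations, follows the active button's target index.
; When that target changes, a second timeline returns it to start at double speed before moving again.
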(event Custom|StartMoving
  (params (reset :type Boolean))
  (bind _platform (Variables|Default|GetPlatform))
  (bind _returnvalue (Transformation|GetWorldLocation _platform))
  (if reset
    (Components|Timeline|SetPlayRate (Variables|Default|GetTimeline) (/ 1.0 (Variables|Default|GetmovementCycleDuration)))
    (if (Variables|Default|GetlastDirection)
      (bind _0_1 (Timeline|Timeline PlayFromStart)
        (:Update
          (Transformation|SetWorldLocation (Variables|Default|GetPlatform) (Math|Vector|Lerp(Vector) (Variables|Default|GetstartLocation) (Variables|Default|GetcurrentTargetLocation) _0_1) false false)
          (if (and (or (Utilities|Operators|EqualEqual _returnvalue (Variables|Default|GetcurrentTargetLocation) 0.0) (Utilities|Operators|EqualEqual _returnvalue (Variables|Default|GetstartLocation) 0.0)) (not reset))
            (Utilities|CustomFlipFlop)))
        (:Finished
          (switch Utilities|FlowControl|Switch|SwitchonBPE_MovingPlatformBehaviour (Variables|Default|Getbehaviour)
            (:NewEnumerator1
              (if (Variables|Default|GetlastDirection)
                (Timeline|Timeline Play)
                (else
                  (Timeline|Timeline Reverse)))))))
      (else
        (Timeline|Timeline ReverseFromEnd)))
    (else
      (Components|Timeline|SetPlayRate (Variables|Default|GetTimeline) (/ 1.0 (Variables|Default|GetmovementCycleDuration)))
      (if (Variables|Default|GetlastDirection)
        (Timeline|Timeline Play)
        (else
          (Timeline|Timeline Reverse))))))

(event Custom|StopMoving
  (bind _platform (Variables|Default|GetPlatform))
  (bind _returnvalue (Transformation|GetWorldLocation _platform))
  (switch Utilities|FlowControl|Switch|SwitchonBPE_MovingPlatformBehaviour (Variables|Default|Getbehaviour)
    (:NewEnumerator0
      (bind _0_1 (Timeline|Timeline Stop)
        (:Update
          (Transformation|SetWorldLocation (Variables|Default|GetPlatform) (Math|Vector|Lerp(Vector) (Variables|Default|GetstartLocation) (Variables|Default|GetcurrentTargetLocation) _0_1) false false)
          (if (and (or (Utilities|Operators|EqualEqual _returnvalue (Variables|Default|GetcurrentTargetLocation) 0.0) (Utilities|Operators|EqualEqual _returnvalue (Variables|Default|GetstartLocation) 0.0)) (not (stale Custom|StartMoving reset)))
            (Utilities|CustomFlipFlop)))
        (:Finished
          (switch Utilities|FlowControl|Switch|SwitchonBPE_MovingPlatformBehaviour (Variables|Default|Getbehaviour)
            (:NewEnumerator1
              (if (Variables|Default|GetlastDirection)
                (Timeline|Timeline Play)
                (else
                  (Timeline|Timeline Reverse))))))))
    (:NewEnumerator1
      (Timeline|Timeline Stop))))

(event Custom|ReturnToStartLocation
  (params (thenStartMoving :type Boolean))
  (Variables|Default|SetlastDirection true)
  (Variables|Default|SetreturnStartLocation (Transformation|GetWorldLocation (Variables|Default|GetPlatform)))
  (Components|Timeline|SetPlayRate (Variables|Default|GetTimelineReturn) (/ 1.0 (/ (Variables|Default|GetmovementCycleDuration) 2.0)))
  (bind _0_1 (Timeline|TimelineReturn PlayFromStart)
    (:Update
      (Transformation|SetWorldLocation (Variables|Default|GetPlatform) (Math|Vector|Lerp(Vector) (Variables|Default|GetreturnStartLocation) (Variables|Default|GetstartLocation) _0_1) false false))
    (:Finished
      (if thenStartMoving
        (CallFunction|StartMoving true)))))

(event EventBeginPlay
  (for _array_element (Variables|Default|GettargetLocations)
    (Utilities|Array|AddUnique (Variables|Default|GettargetLocationsInWord) (Math|Transform|TransformLocation (Transformation|GetActorTransform) _array_element)))
  (Variables|Default|SetstartLocation (Transformation|GetWorldLocation (Variables|Default|GetPlatform)))
  (Variables|Default|SetlastDirection true))

(fn ConstructionScript)

(fn EnableMovingPlatform
  (params (locationIndex :type Integer))
  (bind _activelocationindexes (Variables|Default|GetactiveLocationIndexes))
  (Math|Integer|IncrementInt (Variables|Default|GetcurrentToggledButtons)
    (:%20%20
      (if (Variables|Default|GetswitchLocations)
        (if (not (> (Variables|Default|GetcurrentToggledButtons) 1))
          (if (not (Utilities|Array|ContainsItem _activelocationindexes locationIndex))
            (if (not (> (Utilities|Array|Length _activelocationindexes) 0))
              (Utilities|Array|AddUnique (Variables|Default|GetactiveLocationIndexes) locationIndex)
              (Variables|Default|SetcurrentTargetLocation (Utilities|Array|Get(acopy) (Variables|Default|GettargetLocationsInWord) locationIndex))
              (if (and (!= locationIndex (Variables|Default|GetlastIndex)) (Utilities|Operators|NotEqual(!=) (Transformation|GetWorldLocation (Variables|Default|GetPlatform)) (Variables|Default|GetstartLocation) 0.1))
                (CallFunction|ReturntoStartLocation true)
                (else
                  (CallFunction|StartMoving false)))
              (Variables|Default|SetlastIndex locationIndex :!label _label))))
        (elif (== (Variables|Default|GetcurrentToggledButtons) (Variables|Default|GetbuttonsNeededToEnable))
          (Variables|Default|SetcurrentTargetLocation (Utilities|Array|Get(acopy) (Variables|Default|GettargetLocationsInWord) locationIndex))
          (CallFunction|StartMoving false)
          (goto _label))))))

(fn DisableMovingPlatform
  (params (locationIndex :type Integer))
  (bind _activelocationindexes (Variables|Default|GetactiveLocationIndexes))
  (bind _returnvalue (Utilities|Array|LastIndex _activelocationindexes))
  (bind _output (Utilities|Array|Get(acopy) _activelocationindexes _returnvalue))
  (Math|Integer|DecrementInt (Variables|Default|GetcurrentToggledButtons)
    (:%20%20
      (if (Variables|Default|GetswitchLocations)
        (if (> (Variables|Default|GetcurrentToggledButtons) 0)
          (Utilities|Array|RemoveItem _activelocationindexes locationIndex)
          (if (not (== _output (Variables|Default|GetlastIndex)))
            (Variables|Default|SetcurrentTargetLocation (Utilities|Array|Get(acopy) (Variables|Default|GettargetLocationsInWord) _output))
            (if (Utilities|Operators|NotEqual(!=) (Transformation|GetWorldLocation (Variables|Default|GetPlatform)) (Variables|Default|GetstartLocation) 0.0)
              (CallFunction|ReturntoStartLocation true)
              (else
                (CallFunction|StartMoving false))))
          (else
            (Utilities|Array|Clear (Variables|Default|GetactiveLocationIndexes))
            (Variables|Default|SetcurrentTargetLocation "0, 0, 0" :!label _label)
            (CallFunction|StopMoving)))
        (elif (not (>= (Variables|Default|GetcurrentToggledButtons) (Variables|Default|GetbuttonsNeededToEnable)))
          (goto _label))))))