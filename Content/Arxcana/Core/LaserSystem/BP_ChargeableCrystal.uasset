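; Laser puzzle crystal that, after being charged continuously for ChargeTime, emits a light beam until Duration runs out uncharged, or indefinitely if zero.
; Charge pulses hold a short Charging flag that Tick uses to drive timers and glow.
; CastLight traces each tick, reflecting off mirror materials, reusing beam actors per segment, triggering sensors and charging crystals hit on their RayDetector.
; It can attach to an overlapping moving platform on BeginPlay.
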(event EventCharge
  (Variables|Default|Setcharging true)
  (Utilities|FlowControl|Delay 0.2)
  (Variables|Default|Setcharging false))

(event EventBeginPlay
  (Utilities|FlowControl|Sequence
    (:then_0
      (if (Variables|Default|GetattachToMovingPlatform)
        (CallFunction|AttachtoClosestMovingPlatform)))
    (:then_1
      (Variables|Default|SetcanEmit false)
      (Variables|Default|SetdurationTimer (Variables|Default|Getduration))
      (Components|Activation|SetActive (Variables|Default|GetPointLight) false false))))

(event EventTick
  (params (DeltaSeconds :type Float%20%28single-precision%29))
  (Utilities|FlowControl|Sequence
    (:then_0
      (if (Variables|Default|GetcanEmit)
        (CallFunction|CastLight (Transformation|GetWorldLocation (Variables|Default|GetArrow)) (Math|Vector|GetForwardVector (Variables|Default|GetArrow)) (Variables|Default|GetcastDistance))))
    (:then_1
      (if (Variables|Default|Getcharging)
        (if (not (Variables|Default|GetcanEmit))
          (Variables|Default|SetrunningChargeTimer true))
        (else
          (if (Variables|Default|GetrunningChargeTimer)
            (Variables|Default|SetrunningChargeTimer false)
            (Variables|Default|SetchargeTimer 0.0))
          (if (Variables|Default|GetrunningDurationTimer)
            (bind _output_get (Variables|Default|SetdurationTimer (- (Variables|Default|GetdurationTimer) DeltaSeconds)))
            (if (<= _output_get 0.0)
              (Variables|Default|SetdurationTimer (Variables|Default|Getduration))
              (Variables|Default|SetrunningDurationTimer false)
              (Variables|Default|SetrunningChargeTimer false)
              (Variables|Default|SetchargeTimer 0.0)
              (Variables|Default|SetcanEmit false)
              (CallFunction|StopBeam))))))
    (:then_2
      (if (Variables|Default|GetrunningChargeTimer)
        (bind _output_get_2 (Variables|Default|SetchargeTimer (+ DeltaSeconds (Variables|Default|GetchargeTimer))))
        (if (and (>= _output_get_2 (Variables|Default|GetchargeTime)) (Variables|Default|Getcharging))
          (Variables|Default|SetcanEmit true)
          (Variables|Default|SetrunningChargeTimer false)
          (if (not (== (Variables|Default|Getduration) 0.0))
            (Variables|Default|SetrunningDurationTimer true)))))
    (:then_3
      (if (or (Variables|Default|GetrunningChargeTimer) (Variables|Default|GetrunningDurationTimer))
        (if (== (Rendering|Material|GetMaterial (Variables|Default|GetMesh) 1) (Variables|Default|GetidleMaterial))
          (Rendering|Material|SetMaterial (Variables|Default|GetMesh) 1 (Variables|Default|GetchargeMaterial))
          (Components|Activation|SetActive (Variables|Default|GetPointLight) true false))
        (elif (== (Rendering|Material|GetMaterial (Variables|Default|GetMesh) 1) (Variables|Default|GetchargeMaterial))
          (Rendering|Material|SetMaterial (Variables|Default|GetMesh) 1 (Variables|Default|GetidleMaterial))
          (Components|Activation|SetActive (Variables|Default|GetPointLight) false false))))))

(fn ConstructionScript
  (Variables|Default|SetchargeMaterial "/Game/Arxcana/Art/PuzzleItem/MI_Moon_Crystal_Bright.MI_Moon_Crystal_Bright")
  (Variables|Default|SetidleMaterial "/Game/Arxcana/Art/PuzzleItem/MI_PuzzleItem.MI_PuzzleItem"))

(fn CastLight
  (params (castOrigin :type Vector) (castDirection :type Vector) (castDistance :type Float%20%28double-precision%29))
  (bind _beams (Variables|Default|Getbeams))
  (LocalVariables|SetL_CastOrigin castOrigin)
  (LocalVariables|SetL_CastDirection castDirection)
  (LocalVariables|SetL_CastDistance castDistance)
  (Class|BPISetState|ToggleState(Message) (Variables|Default|GetactivatedSensor) true)
  (LocalVariables|SetL_Continue true)
  (Variables|Default|SetexpectedBeams 1)
  (Variables|Default|SetloopIndex 0)
  (while (LocalVariables|GetL_Continue)
    (Utilities|FlowControl|Sequence
      (:then_0
        (bind (_outhit _returnvalue) (Collision|LineTraceByChannel (LocalVariables|GetL_CastOrigin) (+ (LocalVariables|GetL_CastOrigin) (* (LocalVariables|GetL_CastDirection) (LocalVariables|GetL_CastDistance))) "TraceTypeQuery3" true 0 "None" true "(R=1.000000,G=0.000000,B=0.000000,A=1.000000)" "(R=0.000000,G=1.000000,B=0.000000,A=1.000000)" 0.1))
        (LocalVariables|SetL_BeamStart (LocalVariables|GetL_CastOrigin))
        (if _returnvalue
          (LocalVariables|SetL_BeamEnd (.ImpactPoint (Collision|BreakHitResult _outhit)))
          (if (== (.ReturnValue (Class|PrimitiveComponent|GetMaterialfromCollisionFaceIndex (.HitComponent (Collision|BreakHitResult _outhit)) (.FaceIndex (Collision|BreakHitResult _outhit)))) "/Game/Arxcana/Core/LaserSystem/M_Mirror.M_Mirror")
            (LocalVariables|SetL_CastOrigin (.ImpactPoint (Collision|BreakHitResult _outhit)))
            (LocalVariables|SetL_CastDirection (Math|Vector|MirrorVectorbyNormal (LocalVariables|GetL_CastDirection) (.ImpactNormal (Collision|BreakHitResult _outhit))))
            (LocalVariables|SetL_Continue true)
            (Math|Integer|IncrementInt (Variables|Default|GetexpectedBeams)
              (:%20%20
                _))
            (else
              (if (or (== (.ReturnValue (Class|PrimitiveComponent|GetMaterialfromCollisionFaceIndex (.HitComponent (Collision|BreakHitResult _outhit)) (.FaceIndex (Collision|BreakHitResult _outhit)))) "/Game/Arxcana/Core/LaserSystem/M_LaserSensor_Card.M_LaserSensor_Card") (Utilities|DoesObjectImplementInterface (.HitActor (Collision|BreakHitResult _outhit)) "/Game/Arxcana/Core/Interactables/BPI_SetState.BPI_SetState_C"))
                (Class|BPISetState|ToggleState(Message) (.HitActor (Collision|BreakHitResult _outhit)) true)
                (Variables|Default|SetactivatedSensor (.HitActor (Collision|BreakHitResult _outhit))))
              (LocalVariables|SetL_Continue false :!label _label)))
          (else
            (LocalVariables|SetL_BeamEnd (+ (LocalVariables|GetL_CastOrigin) (* (LocalVariables|GetL_CastDirection) (LocalVariables|GetL_CastDistance))))
            (goto _label)))
        (Math|Integer|IncrementInt (Variables|Default|GetloopIndex)
          (:%20%20
            (if (Utilities|DoesObjectImplementInterface (.HitActor (Collision|BreakHitResult _outhit)) "/Game/Arxcana/Core/Interactables/BPI_Chargeable.BPI_Chargeable_C")
              (bind _asbp_chargeable_crystal (Utilities|Casting|CastToBP_ChargeableCrystal (.HitActor (Collision|BreakHitResult _outhit))))
              (if (== (Variables|BP_ChargeableCrystal_C|GetRayDetector _asbp_chargeable_crystal) (.HitComponent (Collision|BreakHitResult _outhit)))
                (Class|BPIChargeable|Charge(Message) (.HitActor (Collision|BreakHitResult _outhit))))))))
      (:then_1
        (if (< (Utilities|Array|Length (Variables|Default|Getbeams)) (Variables|Default|GetexpectedBeams))
          (bind _returnvalue_2 (Game|SpawnActorfromClass "/Game/Arxcana/Core/LaserSystem/BP_LightBeam_TheSun_NewBeam.BP_LightBeam_TheSun_NewBeam_C" (Math|Transform|MakeTransform "0, 0, 0" "0, 0, 0" "1.000000,1.000000,1.000000") "Undefined" "MultiplyWithRoot" 0 0))
          (Default|SetEnds _returnvalue_2 (LocalVariables|GetL_BeamStart) (LocalVariables|GetL_BeamEnd))
          (Utilities|Array|Add (Variables|Default|Getbeams) _returnvalue_2)
          (Development|PrintString "Spawned a beam")
          (else
            (Default|SetEnds (Utilities|Array|Get(acopy) (Variables|Default|Getbeams) (- (Variables|Default|GetloopIndex) 1)) (LocalVariables|GetL_BeamStart) (LocalVariables|GetL_BeamEnd)))))))
  (if (> (Utilities|Array|Length (Variables|Default|Getbeams)) (Variables|Default|GetexpectedBeams))
    (for _index (range (Variables|Default|GetexpectedBeams) (- (Utilities|Array|Length (Variables|Default|Getbeams)) 1))
      (Actor|DestroyActor (Utilities|Array|Get(acopy) _beams _index))
      (Utilities|Array|RemoveIndex _beams _index))))

(fn StopBeam
  (bind _beams (Variables|Default|Getbeams))
  (for _array_element _beams
    (Actor|DestroyActor _array_element))
  (Utilities|Array|Clear _beams)
  (Class|BPISetState|ToggleState(Message) (Variables|Default|GetactivatedSensor) true))

(fn AttachtoClosestMovingPlatform
  (bind (_outactors _returnvalue) (Collision|SphereOverlapActors (Transformation|GetWorldLocation (Variables|Default|GetMesh)) 5.0 (Utilities|Array|MakeArray (Utilities|Enum|LiteralenumEObjectTypeQuery "ObjectTypeQuery2")) "/Game/Arxcana/Core/Interactables/BP_MovingPlatformNew.BP_MovingPlatformNew_C"))
  (if _returnvalue
    (Transformation|AttachActorToActor (Utilities|Array|Get(acopy) _outactors) "None" "KeepWorld" "KeepWorld" "KeepWorld" true)))