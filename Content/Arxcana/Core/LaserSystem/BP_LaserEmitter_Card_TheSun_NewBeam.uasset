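; Laser emitter for The Sun card that, every tick, fires a light beam toward the point the player's RayDirection component aims at.
; CastLight traces in a loop, reflecting off M_Mirror surfaces, messaging sensors or BPI_SetState actors where it ends, and charging BPI_Chargeable actors it hits.
; Each segment reuses or spawns a beam actor, trimming extras as the path shortens.
; StopBeam destroys all beams and messages the last activated sensor.
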(event EventBeginPlay
  (bind _asbp_main_character (Utilities|Casting|CastToBP_MainCharacter (Game|GetPlayerCharacter 0)))
  (Variables|Default|SetplayerRef _asbp_main_character))

(event EventTick
  (params (DeltaSeconds :type Float%20%28single-precision%29))
  (bind _playerref (Variables|Default|GetplayerRef))
  (bind _raydirection (Variables|/Game/Arxcana/Core/MainCharacter/BP_MainCharacter.BP_MainCharacter_C|GetRayDirection _playerref))
  (bind _returnvalue (Transformation|GetWorldLocation _raydirection))
  (bind (_outhit _returnvalue_2) (Collision|LineTraceByChannel _returnvalue (+ _returnvalue (* (Math|Vector|Normalize (Math|Vector|GetForwardVector (Variables|/Game/Arxcana/Core/MainCharacter/BP_MainCharacter.BP_MainCharacter_C|GetRayDirection (Variables|Default|GetplayerRef)))) (Variables|Default|GetcastDistance))) "TraceTypeQuery1" false 0 "None"))
  (if _returnvalue_2
    (CallFunction|CastLight (Transformation|GetActorLocation self) (- (.ImpactPoint (Collision|BreakHitResult _outhit)) (Transformation|GetActorLocation self)) (Variables|Default|GetcastDistance))
    (else
      (CallFunction|CastLight (Transformation|GetActorLocation self) (- (+ (Transformation|GetWorldLocation (Variables|/Game/Arxcana/Core/MainCharacter/BP_MainCharacter.BP_MainCharacter_C|GetRayDirection (Variables|Default|GetplayerRef))) (* (Math|Vector|Normalize (Math|Vector|GetForwardVector (Variables|/Game/Arxcana/Core/MainCharacter/BP_MainCharacter.BP_MainCharacter_C|GetRayDirection (Variables|Default|GetplayerRef)))) (Variables|Default|GetcastDistance))) (Transformation|GetActorLocation self)) (Variables|Default|GetcastDistance)))))

(fn ConstructionScript)

(fn CastLight
  (params (castOrigin :type Vector) (castDirection :type Vector) (castDistance :type Float%20%28double-precision%29))
  (bind _beams (Variables|Default|Getbeams))
  (LocalVariables|SetL_CastOrigin castOrigin)
  (LocalVariables|SetL_CastDirection castDirection)
  (LocalVariables|SetL_CastDistance castDistance)
  (Class|BPISetState|ToggleState(Message) (Variables|Default|GetactivatedSensor) true)
  (LocalVariables|SetL_Continue true)
  (Variables|Default|SetexpectedBeams 1)
  (Variables|Default|SetloopIndex 0)
  (while (LocalVariables|GetL_Continue)
    (Utilities|FlowControl|Sequence
      (:then_0
        (bind (_outhit _returnvalue) (Collision|LineTraceByChannel (LocalVariables|GetL_CastOrigin) (+ (LocalVariables|GetL_CastOrigin) (* (LocalVariables|GetL_CastDirection) (LocalVariables|GetL_CastDistance))) "TraceTypeQuery3" true 0 "None" true "(R=1.000000,G=0.000000,B=0.000000,A=1.000000)" "(R=0.000000,G=1.000000,B=0.000000,A=1.000000)" 0.1))
        (LocalVariables|SetL_BeamStart (LocalVariables|GetL_CastOrigin))
        (if _returnvalue
          (LocalVariables|SetL_BeamEnd (.ImpactPoint (Collision|BreakHitResult _outhit)))
          (if (== (.ReturnValue (Class|PrimitiveComponent|GetMaterialfromCollisionFaceIndex (.HitComponent (Collision|BreakHitResult _outhit)) (.FaceIndex (Collision|BreakHitResult _outhit)))) "/Game/Arxcana/Core/LaserSystem/M_Mirror.M_Mirror")
            (LocalVariables|SetL_CastOrigin (.ImpactPoint (Collision|BreakHitResult _outhit)))
            (LocalVariables|SetL_CastDirection (Math|Vector|MirrorVectorbyNormal (LocalVariables|GetL_CastDirection) (.ImpactNormal (Collision|BreakHitResult _outhit))))
            (LocalVariables|SetL_Continue true)
            (Math|Integer|IncrementInt (Variables|Default|GetexpectedBeams)
              (:%20%20
                _))
            (else
              (if (or (== (.ReturnValue (Class|PrimitiveComponent|GetMaterialfromCollisionFaceIndex (.HitComponent (Collision|BreakHitResult _outhit)) (.FaceIndex (Collision|BreakHitResult _outhit)))) "/Game/Arxcana/Core/LaserSystem/M_LaserSensor_Card.M_LaserSensor_Card") (Utilities|DoesObjectImplementInterface (.HitActor (Collision|BreakHitResult _outhit)) "/Game/Arxcana/Core/Interactables/BPI_SetState.BPI_SetState_C"))
                (Class|BPISetState|ToggleState(Message) (.HitActor (Collision|BreakHitResult _outhit)) true)
                (Variables|Default|SetactivatedSensor (.HitActor (Collision|BreakHitResult _outhit))))
              (LocalVariables|SetL_Continue false :!label _label)))
          (else
            (LocalVariables|SetL_BeamEnd (+ (LocalVariables|GetL_CastOrigin) (* (LocalVariables|GetL_CastDirection) (LocalVariables|GetL_CastDistance))))
            (goto _label)))
        (Math|Integer|IncrementInt (Variables|Default|GetloopIndex)
          (:%20%20
            (if (Utilities|DoesObjectImplementInterface (.HitActor (Collision|BreakHitResult _outhit)) "/Game/Arxcana/Core/Interactables/BPI_Chargeable.BPI_Chargeable_C")
              (Class|BPIChargeable|Charge(Message) (.HitActor (Collision|BreakHitResult _outhit)))))))
      (:then_1
        (if (< (Utilities|Array|Length (Variables|Default|Getbeams)) (Variables|Default|GetexpectedBeams))
          (bind _returnvalue_2 (Game|SpawnActorfromClass "/Game/Arxcana/Core/LaserSystem/BP_LightBeam_TheSun_NewBeam.BP_LightBeam_TheSun_NewBeam_C" (Math|Transform|MakeTransform "0, 0, 0" "0, 0, 0" "1.000000,1.000000,1.000000") "Undefined" "MultiplyWithRoot" 0 0))
          (Default|SetEnds _returnvalue_2 (LocalVariables|GetL_BeamStart) (LocalVariables|GetL_BeamEnd))
          (Utilities|Array|Add (Variables|Default|Getbeams) _returnvalue_2)
          (Development|PrintString "Spawned a beam")
          (else
            (Default|SetEnds (Utilities|Array|Get(acopy) (Variables|Default|Getbeams) (- (Variables|Default|GetloopIndex) 1)) (LocalVariables|GetL_BeamStart) (LocalVariables|GetL_BeamEnd)))))))
  (if (> (Utilities|Array|Length (Variables|Default|Getbeams)) (Variables|Default|GetexpectedBeams))
    (for _index (range (Variables|Default|GetexpectedBeams) (- (Utilities|Array|Length (Variables|Default|Getbeams)) 1))
      (Actor|DestroyActor (Utilities|Array|Get(acopy) _beams _index))
      (Utilities|Array|RemoveIndex _beams _index))))

(fn StopBeam
  (bind _beams (Variables|Default|Getbeams))
  (for _array_element _beams
    (Actor|DestroyActor _array_element))
  (Utilities|Array|Clear _beams)
  (Class|BPISetState|ToggleState(Message) (Variables|Default|GetactivatedSensor) true))