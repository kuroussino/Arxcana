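; Planetary laser emitter for The Moon that casts a light beam from its arrow and bounces it off mirrors.
; Tick, behind a short Delay, destroys the old beams and retraces the path, reflecting at M_Mirror surfaces until another surface or a miss.
; Each segment spawns a BP_LightBeam_TheMoon actor.
; An M_LaserSensor_Planetary hit is stored and sent a toggle message, repeated on each recast and in StopBeam.
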(event EventTick
  (params (DeltaSeconds :type Float%20%28single-precision%29))
  (bind _arrow (Variables|Default|GetArrow))
  (Utilities|FlowControl|Delay 0.01)
  (CallFunction|CastLight (Transformation|GetWorldLocation _arrow) (Math|Vector|GetForwardVector _arrow) (Variables|Default|GetcastDistance)))

(fn ConstructionScript)

(fn CastLight
  (params (castOrigin :type Vector) (castDirection :type Vector) (castDistance :type Float%20%28double-precision%29))
  (bind _beams (Variables|Default|Getbeams))
  (LocalVariables|SetL_CastOrigin castOrigin)
  (LocalVariables|SetL_CastDirection castDirection)
  (LocalVariables|SetL_CastDistance castDistance)
  (for _array_element _beams
    (Actor|DestroyActor _array_element))
  (Utilities|Array|Clear _beams)
  (Class|BPISetState|ToggleState(Message) (Variables|Default|GetactivatedSensor) false)
  (while (LocalVariables|GetL_Continue)
    (Utilities|FlowControl|Sequence
      (:then_0
        (bind (_outhit _returnvalue) (Collision|LineTraceByChannel (LocalVariables|GetL_CastOrigin) (+ (LocalVariables|GetL_CastOrigin) (* (LocalVariables|GetL_CastDirection) (LocalVariables|GetL_CastDistance))) "TraceTypeQuery3" true 0 "ForDuration" true "(R=1.000000,G=0.000000,B=0.000000,A=1.000000)" "(R=0.000000,G=1.000000,B=0.000000,A=1.000000)" 0.1))
        (LocalVariables|SetL_BeamStart (LocalVariables|GetL_CastOrigin))
        (if _returnvalue
          (LocalVariables|SetL_BeamEnd (.ImpactPoint (Collision|BreakHitResult _outhit)))
          (if (== (.ReturnValue (Class|PrimitiveComponent|GetMaterialfromCollisionFaceIndex (.HitComponent (Collision|BreakHitResult _outhit)) (.FaceIndex (Collision|BreakHitResult _outhit)))) "/Game/Arxcana/Core/LaserSystem/M_Mirror.M_Mirror")
            (LocalVariables|SetL_CastOrigin (.ImpactPoint (Collision|BreakHitResult _outhit)))
            (LocalVariables|SetL_CastDirection (Math|Vector|MirrorVectorbyNormal (LocalVariables|GetL_CastDirection) (.ImpactNormal (Collision|BreakHitResult _outhit))))
            (LocalVariables|SetL_Continue true)
            (else
              (if (== (.ReturnValue (Class|PrimitiveComponent|GetMaterialfromCollisionFaceIndex (.HitComponent (Collision|BreakHitResult _outhit)) (.FaceIndex (Collision|BreakHitResult _outhit)))) "/Game/Arxcana/Core/LaserSystem/M_LaserSensor_Planetary.M_LaserSensor_Planetary")
                (Class|BPISetState|ToggleState(Message) (.HitActor (Collision|BreakHitResult _outhit)) false)
                (Variables|Default|SetactivatedSensor (.HitActor (Collision|BreakHitResult _outhit))))
              (LocalVariables|SetL_Continue false :!label _label)))
          (else
            (LocalVariables|SetL_BeamEnd (+ (LocalVariables|GetL_CastOrigin) (* (LocalVariables|GetL_CastDirection) (LocalVariables|GetL_CastDistance))))
            (goto _label))))
      (:then_1
        (bind _returnvalue_2 (Game|SpawnActorfromClass "/Game/Arxcana/Core/LaserSystem/BP_LightBeam_TheMoon.BP_LightBeam_TheMoon_C" (Math|Transform|MakeTransform "0, 0, 0" "0, 0, 0" "1.000000,1.000000,1.000000") "Undefined" "MultiplyWithRoot" 0 0))
        (Default|SetEnds _returnvalue_2 (LocalVariables|GetL_BeamStart) (LocalVariables|GetL_BeamEnd))
        (Utilities|Array|Add (Variables|Default|Getbeams) _returnvalue_2)))))

(fn StopBeam
  (bind _beams (Variables|Default|Getbeams))
  (for _array_element _beams
    (Actor|DestroyActor _array_element))
  (Utilities|Array|Clear _beams)
  (Class|BPISetState|ToggleState(Message) (Variables|Default|GetactivatedSensor) false))