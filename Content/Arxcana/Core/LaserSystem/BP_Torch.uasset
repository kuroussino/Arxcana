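; BP_Torch is a torch in the laser system that switches its flames and point light on or off together.
; On BeginPlay it applies its initial state from StartEnabled.
; TurnOn, TurnOff and ToggleState share the same two paths, which activate or deactivate the Flames, set PointLight visibility, then call CallActiveCheck after every change.
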(event Custom|TurnOn
  (Components|Activation|Activate (Variables|Default|GetFlames) false)
  (Rendering|SetVisibility (Variables|Default|GetPointLight) true false)
  (Default|CallActiveCheck))

(event Custom|TurnOff
  (Components|Activation|Deactivate (Variables|Default|GetFlames))
  (Rendering|SetVisibility (Variables|Default|GetPointLight) false false)
  (Default|CallActiveCheck))

(event EventBeginPlay
  (if (Variables|Default|GetstartEnabled)
    (CallFunction|Turnon)
    (else
      (CallFunction|TurnOff))))

(event EventToggleState
  (params (On/Off :type Boolean))
  (bind _flames (Variables|Default|GetFlames))
  (bind _pointlight (Variables|Default|GetPointLight))
  (if On/Off
    (Components|Activation|Activate _flames false)
    (Rendering|SetVisibility _pointlight true false)
    (else
      (Components|Activation|Deactivate _flames)
      (Rendering|SetVisibility _pointlight false false)))
  (Default|CallActiveCheck))

(fn ConstructionScript)