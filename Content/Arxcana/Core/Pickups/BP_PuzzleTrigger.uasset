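; BP_PuzzleTrigger is a card pickup that can also start a puzzle, with its mesh bobbing on two alternating timelines.
; On player overlap, it adds its card to BP_MainCharacter, refreshes or briefly shows the card carousel, then destroys itself.
; When flagged, it also sends a puzzle trigger message and closes its related door.
; TriggerPuzzle only prints debug text, and ToggleTorches, which messages linked lights, is not called here.
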(event OnComponentBeginOverlap(Box)
  (params (OverlappedComponent :type Primitive%20Component%20Object%20Reference) (OtherActor :type Actor%20Object%20Reference) (OtherComp :type Primitive%20Component%20Object%20Reference) (OtherBodyIndex :type Integer) (bFromSweep :type Boolean) (SweepResult :type Hit%20Result%20Structure%20%28by%20ref%29))
  (bind _returnvalue (Game|GetPlayerCharacter 0))
  (bind _relateddoor (Variables|Default|GetrelatedDoor))
  (if (== OtherActor _returnvalue)
    (bind _asbp_main_character (Utilities|Casting|CastToBP_MainCharacter _returnvalue))
    (Default|AddCard _asbp_main_character (Variables|Default|GetcardType))
    (if (Variables|Default|GetneedsToTriggerPuzzle)
      (Class|BPITriggerPuzzle|TriggerPuzzle(Message) self)
      (Utilities|IsValid _relateddoor
        (:Is%20Valid
          (Default|CloseDoor _relateddoor))
        (:Is%20Not%20Valid
          _)))
    (if (Utilities|IsValid (Variables|/Game/Arxcana/Core/MainCharacter/BP_MainCharacter.BP_MainCharacter_C|GetcardCarousel _asbp_main_character))
      (Default|RefreshCarousel _asbp_main_character)
      (else
        (Default|TimedShwCarousel _asbp_main_character (Variables|Default|GettimedCarouselDuration))))
    (if (Utilities|Enum|NotEqual(Enum) (Variables|Default|GetcardType) "NewEnumerator0")
      _
      (else
        _))
    (Actor|DestroyActor)))

(event EventTriggerPuzzle
  (Development|PrintString "Puzzle triggered!"))

(event EventBeginPlay
  (bind _0_1 (Timeline|FloatingUp Play)
    (:Update
      (Transformation|SetRelativeLocation (Variables|Default|GetStaticMesh) (Math|Vector|MakeVector 0.0 0.0 (* _0_1 1e+01)) false false))
    (:Finished
      (bind _1_0 (Timeline|FloatingDown PlayFromStart)
        (:Update
          (Transformation|SetRelativeLocation (Variables|Default|GetStaticMesh) (Math|Vector|MakeVector 0.0 0.0 (* _1_0 1e+01)) false false))
        (:Finished
          (Timeline|FloatingUp PlayFromStart))))))

(fn ConstructionScript)

(fn ToggleTorches
  (params (on/off :type Boolean))
  (for _array_element (Variables|Default|Getlights)
    (Class|BPISetState|ToggleState(Message) _array_element on/off)))