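; Five-ring planetary "Sun" puzzle that fires a laser beam when every ring reaches its correct state.
; EnablePlanetary moves rings from idle to start rotations, and ChangeRingsState steps the given rings through their RingStates rotations.
; A shared timeline lerps rings along the shortest path, using a sentinel rotation to skip unaffected ones.
; On finish it compares state indexes, not rotations, to the solution and spawns or destroys the laser emitter.
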(event Custom|ChangeRingsRotations
  (params (speedModifier :type Float%20%28double-precision%29))
  (bind _rotationtimeline (Variables|Default|GetRotationTimeline))
  ;[0.2961 0 0] Change Rings Rotations
  (Components|Timeline|SetPlayRate _rotationtimeline (* (/ 1.0 (Variables|Default|GetringRotationSpeed)) speedModifier))
  (Components|Timeline|SetNewTime _rotationtimeline (Variables|Default|GettimelineStartOfsset))
  (bind _0_1 (Timeline|RotationTimeline PlayFromStart)
    (:Update
      (for (_array_element _array_index) (Variables|Default|Getrings)
        (if (and (Utilities|Operators|NotEqual(!=) (Utilities|Array|Get(acopy) (Variables|Default|GetcurrStartRotations) _array_index) "1.000000,1.000000,1.000000" 0.0) (Utilities|Operators|NotEqual(!=) (Utilities|Array|Get(acopy) (Variables|Default|GetcurrStopRotations) _array_index) "1.000000,1.000000,1.000000" 0.0))
          (Transformation|SetRelativeRotation _array_element (Math|Rotator|Lerp(Rotator) (Utilities|Array|Get(acopy) (Variables|Default|GetcurrStartRotations) _array_index) (Utilities|Array|Get(acopy) (Variables|Default|GetcurrStopRotations) _array_index) _0_1 true) false false))))
    (:Finished
      (CallFunction|ClearStartEndArrays)
      (CallFunction|CheckPuzzleSolution))))

(event EventBeginPlay
  (if (not (Variables|Default|GetisHologram))
    (CallFunction|InitializeRingStatesIndexes)
    (CallFunction|PopulateRingsArray)
    (CallFunction|SetupIdleRingsPosition)))

(fn ConstructionScript)

(fn EnablePlanetary
  (CallFunction|PopulateStartEndArrays)
  (switch Utilities|FlowControl|Switch|SwitchonBPE_PlanetaryStartPosition (Variables|Default|GetstartPosition)
    (:NewEnumerator0
      (for _index (range 0 4)
        (Utilities|Array|SetArrayElem (Variables|Default|GetcurrStartRotations) _index (Variables|/Script/Engine.SceneComponent|GetRelativeRotation (Utilities|Array|Get(acopy) (Variables|Default|Getrings) _index)))
        (Utilities|Array|SetArrayElem (Variables|Default|GetcurrStopRotations) _index (Math|Rotator|MakeRotator (Math|Random|RandomFloatinRange 0.0 3.6e+02) (Math|Random|RandomFloatinRange 0.0 3.6e+02) (Math|Random|RandomFloatinRange (- 0.0 (Variables|Default|GetillegalRotAngle)) (- 3.6e+02 (Variables|Default|GetillegalRotAngle)))))))
    (:NewEnumerator1
      (for _index_2 (range 0 4)
        (Utilities|Array|SetArrayElem (Variables|Default|GetcurrStartRotations) _index_2 (Variables|/Script/Engine.SceneComponent|GetRelativeRotation (Utilities|Array|Get(acopy) (Variables|Default|Getrings) _index_2)))
        (Utilities|Array|SetArrayElem (Variables|Default|GetcurrStopRotations) _index_2 "0.000000,90.000000,90.000000"))))
  (CallFunction|ChangeRingsRotations 0.25)
  (Variables|Default|SetneedsToFireLaser true))

(fn PopulateRingsArray
  (Utilities|Array|Add (Variables|Default|Getrings) (Variables|Default|GetRing_1))
  (Utilities|Array|Add (Variables|Default|Getrings) (Variables|Default|GetRing_2))
  (Utilities|Array|Add (Variables|Default|Getrings) (Variables|Default|GetRing_3))
  (Utilities|Array|Add (Variables|Default|Getrings) (Variables|Default|GetRing_4))
  (Utilities|Array|Add (Variables|Default|Getrings) (Variables|Default|GetRing_5)))

(fn InitializeRingStatesIndexes
  (for _index (range 0 4)
    (Utilities|Array|Add (Variables|Default|GetringStatesIndexes) -1)))

(fn ChangeRingsState
  (params (affectedRings :type Array%20of%20Integers))
  (bind _ringstatesindexes (Variables|Default|GetringStatesIndexes))
  (if (Utilities|Array|IsNotEmpty affectedRings)
    (CallFunction|PopulateStartEndArrays)
    (for _array_element affectedRings
      (if (and (== (Utilities|Array|Get(acopy) _ringstatesindexes (- _array_element 1)) 0) (== (Utilities|Array|Length (Utilities|Struct|BreakSTR_RingRotations (.Value (Utilities|Map|Find (Variables|Default|GetringStates) _array_element)))) 1))
        _
        (elif (>= (+ (Utilities|Array|Get(acopy) _ringstatesindexes (- _array_element 1)) 1) (Utilities|Array|Length (Utilities|Struct|BreakSTR_RingRotations (.Value (Utilities|Map|Find (Variables|Default|GetringStates) _array_element)))))
          (Utilities|Array|SetArrayElem _ringstatesindexes (- _array_element 1) 0)
          (else
            (Math|Integer|IncrementInt (Utilities|Array|Get(acopy) _ringstatesindexes (- _array_element 1))
              (:%20%20
                _)))))
      (Utilities|Array|SetArrayElem (Variables|Default|GetcurrStartRotations) (- _array_element 1) (Variables|/Script/Engine.SceneComponent|GetRelativeRotation (Utilities|Array|Get(acopy) (Variables|Default|Getrings) (- _array_element 1))))
      (Utilities|Array|SetArrayElem (Variables|Default|GetcurrStopRotations) (- _array_element 1) (Utilities|Array|Get(acopy) (Utilities|Struct|BreakSTR_RingRotations (.Value (Utilities|Map|Find (Variables|Default|GetringStates) _array_element))) (Utilities|Array|Get(acopy) _ringstatesindexes (- _array_element 1))))
      (Development|PrintString (Utilities|String|Append (Utilities|String|ToString(Integer) _array_element) (Utilities|String|ToString(Rotator) (Utilities|Array|Get(acopy) (Utilities|Struct|BreakSTR_RingRotations (.Value (Utilities|Map|Find (Variables|Default|GetringStates) _array_element))) (Utilities|Array|Get(acopy) _ringstatesindexes (- _array_element 1)))))))
    (CallFunction|ChangeRingsRotations 1.0)))

(fn ClearStartEndArrays
  (Utilities|Array|Clear (Variables|Default|GetcurrStartRotations))
  (Utilities|Array|Clear (Variables|Default|GetcurrStopRotations)))

(fn PopulateStartEndArrays
  (for _index (range 0 4)
    (Utilities|Array|Add (Variables|Default|GetcurrStartRotations) "1.000000,1.000000,1.000000")
    (Utilities|Array|Add (Variables|Default|GetcurrStopRotations) "1.000000,1.000000,1.000000")))

(fn SetupIdleRingsPosition
  (switch Utilities|FlowControl|Switch|SwitchonBPE_PlanetaryStartPosition (Variables|Default|GetstartPosition)
    (:NewEnumerator0
      (for _index (range 0 4)
        (Transformation|SetRelativeRotation (Utilities|Array|Get(acopy) (Variables|Default|Getrings) _index) "0.000000,90.000000,90.000000" false false)))
    (:NewEnumerator1
      (for _index_2 (range 0 4)
        (Transformation|SetRelativeRotation (Utilities|Array|Get(acopy) (Variables|Default|Getrings) _index_2) (Math|Random|RandomRotator false) false false)))))

(fn ToggleBeam
  (params (active :type Boolean))
  (bind _beamspawnpoint (Variables|Default|GetBeamSpawnPoint))
  (bind _returnvalue (Transformation|GetWorldTransform _beamspawnpoint))
  (if active
    (bind _returnvalue_2 (Game|SpawnActorfromClass "/Game/Arxcana/Core/LaserSystem/BP_LaserEmitter_Planetary_TheSun.BP_LaserEmitter_Planetary_TheSun_C" (Math|Transform|MakeTransform (.location _returnvalue) (.rotation _returnvalue) "1.000000,1.000000,1.000000") "Undefined" "MultiplyWithRoot" 0 0))
    (bind _output_get (Variables|Default|SetcurrentBeam _returnvalue_2))
    (Transformation|AttachComponentToComponent _output_get _beamspawnpoint "None" "KeepWorld" "KeepWorld" "KeepWorld" true)
    (Variables|/Game/Arxcana/Core/LaserSystem/BP_LaserEmitter_Planetary_TheSun.BP_LaserEmitter_Planetary_TheSun_C|Setemitting (Variables|Default|GetcurrentBeam) true)
    (else
      (Default|StopBeam (Variables|Default|GetcurrentBeam))
      (Variables|/Game/Arxcana/Core/LaserSystem/BP_LaserEmitter_Planetary_TheSun.BP_LaserEmitter_Planetary_TheSun_C|Setemitting (Variables|Default|GetcurrentBeam) false)
      (Actor|DestroyActor (Variables|Default|GetcurrentBeam))
      (Variables|Default|SetcurrentBeam 0))))

(fn CheckPuzzleSolution
  (Variables|Default|SetcurrCorrectRings 0)
  (for (_array_element _array_index) (Variables|Default|GetringStatesIndexes)
    (if (== (- (Utilities|Array|Get(acopy) (Variables|Default|GetcorrectFinalIndexes) _array_index) 1) _array_element)
      (Math|Integer|IncrementInt (Variables|Default|GetcurrCorrectRings))))
  (if (== (Variables|Default|GetcurrCorrectRings) 5)
    (CallFunction|ToggleBeam true)
    (elif (Variables|/Game/Arxcana/Core/LaserSystem/BP_LaserEmitter_Planetary_TheSun.BP_LaserEmitter_Planetary_TheSun_C|Getemitting (Variables|Default|GetcurrentBeam))
      (CallFunction|ToggleBeam false))))