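; BP_SwitchArea is a trigger zone that tells the player character which switchable objects it can affect while inside it.
; When the player enters TriggerArea, it gathers the overlapping BP_SwitchableObject actors and assigns them to the SwitchableActors list on BP_MainCharacter.
; The list is a snapshot taken on entry, and it is cleared when the player leaves.
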(event OnComponentBeginOverlap(TriggerArea)
  (params (OverlappedComponent :type Primitive%20Component%20Object%20Reference) (OtherActor :type Actor%20Object%20Reference) (OtherComp :type Primitive%20Component%20Object%20Reference) (OtherBodyIndex :type Integer) (bFromSweep :type Boolean) (SweepResult :type Hit%20Result%20Structure%20%28by%20ref%29))
  (Utilities|CheckIsPlayer OtherActor
    (:true
      (bind _asbp_main_character (Utilities|Casting|CastToBP_MainCharacter OtherActor))
      (bind _switchableobjects (CallFunction|GetSwitchableObjects))
      (Variables|/Game/Arxcana/Core/MainCharacter/BP_MainCharacter.BP_MainCharacter_C|SetswitchableActors _asbp_main_character _switchableobjects))))

(event OnComponentEndOverlap(TriggerArea)
  (params (OverlappedComponent :type Primitive%20Component%20Object%20Reference) (OtherActor :type Actor%20Object%20Reference) (OtherComp :type Primitive%20Component%20Object%20Reference) (OtherBodyIndex :type Integer))
  (Utilities|CheckIsPlayer OtherActor
    (:true
      (bind _asbp_main_character (Utilities|Casting|CastToBP_MainCharacter OtherActor))
      (Utilities|Array|Clear (Variables|/Game/Arxcana/Core/MainCharacter/BP_MainCharacter.BP_MainCharacter_C|GetswitchableActors _asbp_main_character)))))

(event EventBeginPlay)

(event Collision|EventActorBeginOverlap
  (params (OtherActor :type Actor%20Object%20Reference)))

(event EventTick
  (params (DeltaSeconds :type Float%20%28single-precision%29)))

(fn ConstructionScript)

(fn GetSwitchableObjects
  (return (Collision|GetOverlappingActors (Variables|Default|GetTriggerArea) "/Game/Arxcana/Core/SwitchableObjects/BP_SwitchableObject.BP_SwitchableObject_C" :!class /Script/Engine.PrimitiveComponent)))