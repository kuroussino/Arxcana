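; Switchable world object that is solid only when the global state matches its ActiveState, starting from the main character's GlobalState at BeginPlay.
; EnterChangingState reveals the mesh with a supplied enabled or disabled material and sets Pawn collision to match.
; SwitchState updates that material and collision only while changing.
; ExitChangingState restores the original material cached in construction, hiding inactive objects and toggling Pawn and custom trace collision.
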(event EventBeginPlay
  (bind _asbp_main_character (Utilities|Casting|CastToBP_MainCharacter (Game|GetPlayerCharacter 0)))
  (CallFunction|ExitChangingState (Variables|/Game/Arxcana/Core/MainCharacter/BP_MainCharacter.BP_MainCharacter_C|GetglobalState _asbp_main_character)))

(event Collision|EventActorBeginOverlap
  (params (OtherActor :type Actor%20Object%20Reference)))

(event EventTick
  (params (DeltaSeconds :type Float%20%28single-precision%29)))

(event EventSwitchState
  (params (globalState :type BPE_HighPriestressState%20Enum :default "NewEnumerator0"))
  (bind _mesh (Variables|Default|GetMesh))
  (bind _mesh_2 (Variables|Default|GetMesh))
  (if (Variables|Default|GetchangingState)
    (if (Utilities|Enum|Equal(Enum) globalState (Variables|Default|GetactiveState))
      (Rendering|Material|SetMaterial _mesh 0 (Variables|Default|GetenabledMatRef))
      (Collision|SetCollisionResponsetoChannel _mesh "ECC_Pawn" "ECR_Block")
      (else
        (Rendering|Material|SetMaterial _mesh_2 0 (Variables|Default|GetdisabledMatRef))
        (Collision|SetCollisionResponsetoChannel _mesh_2 "ECC_Pawn" "ECR_Ignore")))))

(fn ConstructionScript
  (Variables|Default|SetobjectMaterial (Rendering|Material|GetMaterial (Variables|Default|GetMesh) 0)))

(fn EnterChangingState
  (params (globalState :type BPE_HighPriestressState%20Enum :default "NewEnumerator0") (enabledMaterial :type Material%20Interface%20Object%20Reference) (disabledMaterial :type Material%20Interface%20Object%20Reference))
  (bind _mesh (Variables|Default|GetMesh))
  (bind _activestate (Variables|Default|GetactiveState))
  (bind _returnvalue (Utilities|Enum|Equal(Enum) globalState _activestate))
  (bind _output_get (Variables|Default|SetenabledMatRef enabledMaterial))
  (bind _output_get_2 (Variables|Default|SetdisabledMatRef disabledMaterial))
  (if _returnvalue
    (Rendering|Material|SetMaterial (Variables|Default|GetMesh) 0 _output_get)
    (else
      (Rendering|Material|SetMaterial (Variables|Default|GetMesh) 0 _output_get_2)))
  (Variables|Default|SetchangingState true)
  (Rendering|SetVisibility _mesh true false)
  (if _returnvalue
    (Collision|SetCollisionResponsetoChannel _mesh "ECC_Pawn" "ECR_Block")
    (else
      (Collision|SetCollisionResponsetoChannel _mesh "ECC_Pawn" "ECR_Ignore")))
  (Development|PrintString "entered changin state"))

(fn ExitChangingState
  (params (globalState :type BPE_HighPriestressState%20Enum :default "NewEnumerator0"))
  (bind _mesh (Variables|Default|GetMesh))
  (bind _mesh_2 (Variables|Default|GetMesh))
  (if (Utilities|Enum|Equal(Enum) globalState (Variables|Default|GetactiveState))
    (Rendering|SetVisibility _mesh true false)
    (Collision|SetCollisionResponsetoChannel _mesh "ECC_Pawn" "ECR_Block")
    (Collision|SetCollisionResponsetoChannel _mesh "ECC_GameTraceChannel1" "ECR_Block")
    (else
      (Rendering|SetVisibility _mesh_2 false false)
      (Collision|SetCollisionResponsetoChannel _mesh_2 "ECC_Pawn" "ECR_Ignore")
      (Collision|SetCollisionResponsetoChannel _mesh_2 "ECC_GameTraceChannel1" "ECR_Ignore")))
  (Rendering|Material|SetMaterial (Variables|Default|GetMesh) 0 (Variables|Default|GetobjectMaterial))
  (Variables|Default|SetchangingState false)
  (Development|PrintString "leaving changing state"))