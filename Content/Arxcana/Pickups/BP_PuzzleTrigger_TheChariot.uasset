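; Puzzle trigger for The Chariot card, a child of a parent puzzle trigger class, that removes a blocking actor from the level.
; On BeginPlay it sets its CardType to the enum entry for this variant.
; Its TriggerPuzzle override runs the parent logic, then destroys the referenced BlockToRemove actor if it is valid.
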(event EventBeginPlay
  (Variables|Default|SetcardType "NewEnumerator2"))

(event Collision|EventActorBeginOverlap
  (params (OtherActor :type Actor%20Object%20Reference))
  (|CallParentFunction OtherActor) ; This node is disabled and will not be called.\nDrag off pins to build functionality.
)

(event EventTick
  (params (DeltaSeconds :type Float%20%28single-precision%29))
  (|CallParentFunction DeltaSeconds) ; This node is disabled and will not be called.\nDrag off pins to build functionality.
)

(event EventTriggerPuzzle
  (bind _blocktoremove (Variables|Default|GetblockToRemove))
  (|CallParentFunction)
  (Utilities|IsValid _blocktoremove
    (:Is%20Valid
      (Actor|DestroyActor _blocktoremove))))

(fn ConstructionScript
  (|CallParentFunction))