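; Puzzle trigger pickup for The Magician card, a child Blueprint that specializes a parent puzzle trigger.
; On BeginPlay it sets its card type enum.
; When the puzzle triggers, it runs the parent logic, then calls ShowWall on its referenced breakable wall.
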(event EventBeginPlay
  (Variables|Default|SetcardType "NewEnumerator3"))

(event Collision|EventActorBeginOverlap
  (params (OtherActor :type Actor%20Object%20Reference))
  (|CallParentFunction OtherActor) ; This node is disabled and will not be called.\nDrag off pins to build functionality.
)

(event EventTick
  (params (DeltaSeconds :type Float%20%28single-precision%29))
  (|CallParentFunction DeltaSeconds) ; This node is disabled and will not be called.\nDrag off pins to build functionality.
)

(event EventTriggerPuzzle
  (|CallParentFunction)
  (Default|ShowWall (Variables|Default|GetbreakableWall)))

(fn ConstructionScript
  (|CallParentFunction))