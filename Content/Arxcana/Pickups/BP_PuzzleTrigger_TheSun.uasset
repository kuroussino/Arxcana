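; Puzzle trigger pickup for The Sun card, a child Blueprint that toggles torches when its puzzle is triggered.
; BeginPlay sets the card type to its enum value.
; The TriggerPuzzle override runs the parent logic, then calls ToggleTorches with the Onoff value as this card's puzzle-specific effect.
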(event EventBeginPlay
  (Variables|Default|SetcardType "NewEnumerator0"))

(event Collision|EventActorBeginOverlap
  (params (OtherActor :type Actor%20Object%20Reference))
  (|CallParentFunction OtherActor) ; This node is disabled and will not be called.\nDrag off pins to build functionality.
)

(event EventTick
  (params (DeltaSeconds :type Float%20%28single-precision%29))
  (|CallParentFunction DeltaSeconds) ; This node is disabled and will not be called.\nDrag off pins to build functionality.
)

(event EventTriggerPuzzle
  (|CallParentFunction)
  (CallFunction|ToggleTorches (Variables|Default|Geton/off)) ; Depends on the puzzle
)

(fn ConstructionScript
  (|CallParentFunction))