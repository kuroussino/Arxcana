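; BP_TutorialText is a tutorial text actor that bobs vertically in the world.
; The construction script sets its Text component's content and material from the TextToPrint and Material variables.
; On BeginPlay, two timelines drive the text's relative Z and restart each other on finish, producing an endless looping hover without using Tick.
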(event EventBeginPlay
  (bind _0_1 (Timeline|Timeline Play)
    (:Update
      (Transformation|SetRelativeLocation (Variables|Default|GetText) (Math|Vector|MakeVector 0.0 0.0 (* _0_1 7.5)) false false))
    (:Finished
      (bind _1_0 (Timeline|Timeline_0 PlayFromStart)
        (:Update
          (Transformation|SetRelativeLocation (Variables|Default|GetText) (Math|Vector|MakeVector 0.0 0.0 (* _1_0 7.5)) false false))
        (:Finished
          (Timeline|Timeline PlayFromStart))))))

(event Collision|EventActorBeginOverlap
  (params (OtherActor :type Actor%20Object%20Reference)))

(event EventTick
  (params (DeltaSeconds :type Float%20%28single-precision%29)))

(fn ConstructionScript
  (bind _text (Variables|Default|GetText))
  (Rendering|Components|TextRender|SetText _text (Variables|Default|GetTextToPrint))
  (Class|TextRenderComponent|SetTextMaterial _text (Variables|Default|GetMaterial)))