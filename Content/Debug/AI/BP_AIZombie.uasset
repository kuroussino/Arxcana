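; BP_AIZombie is a debug zombie AI that walks an ordered patrol route and prints a loss message when it completes it.
; BeginPlay caches patrol actor locations, then RandomRoam uses AI MoveTo sequentially, despite its name, calling itself after each success.
; AddPatrolPoint distracts the zombie by inserting a location at the current index and restarting movement.
; The Distracted flag has no effect on movement, and its reset is unreachable.
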(event Custom|AddPatrolPoint
  (params (patrolPoint :type Vector))
  (bind _actualpatrolpoints (Variables|Default|GetactualPatrolPoints))
  (bind _result (Math|Integer|DecrementInt (Utilities|Array|Length _actualpatrolpoints))
    (:%20%20
      (Utilities|Array|Add _actualpatrolpoints (Utilities|Array|Get(acopy) _actualpatrolpoints _result))
      (Utilities|Array|Insert _actualpatrolpoints patrolPoint (+ (Variables|Default|GetcurrentPatrolIndex) 0))
      (Variables|Default|Setdistracted true)
      (CallFunction|RandomRoam))))

(event Custom|RandomRoam
  (if (Variables|Default|Getdistracted)
    _
    (else
      _))
  (bind _output_get (Variables|Default|SetcurrentPatrolPoint (Utilities|Array|Get(acopy) (Variables|Default|GetactualPatrolPoints) (Variables|Default|GetcurrentPatrolIndex))))
  (AI|AIMoveTo self _output_get 0 5.0 false
    (:OnSuccess
      (Math|Integer|IncrementInt (Variables|Default|GetcurrentPatrolIndex)
        (:%20%20
          (Variables|Default|SetcurrentPatrolIndex (Variables|Default|GetcurrentPatrolIndex))
          (if (< (Variables|Default|GetcurrentPatrolIndex) (Utilities|Array|Length (Variables|Default|GetactualPatrolPoints)))
            (Development|PrintString (Utilities|String|Append "GOING TO: " (Utilities|String|ToString(Vector) (Utilities|Array|Get(acopy) (Variables|Default|GetactualPatrolPoints) (Variables|Default|GetcurrentPatrolIndex)))))
            (CallFunction|RandomRoam)
            (else
              (Development|PrintString "YOU LOST!"))))))))

(event EventBeginPlay
  (Development|PrintString "STARTED")
  (for _array_element (Variables|Default|GetpatrolPoints)
    (Utilities|Array|Add (Variables|Default|GetactualPatrolPoints) (Transformation|GetActorLocation _array_element)))
  (Variables|Default|SetcurrentPatrolIndex 0)
  (CallFunction|RandomRoam))

(fn ConstructionScript)