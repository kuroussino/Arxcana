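; BP_WarpManager is a debug actor that steps the player through a list of warp locations, then opens the main hub level.
; When Active, BeginPlay registers itself on the player's BP_MainCharacter as WarpManager and warps to the first entry.
; Each WarpToNextLevel call teleports the player to the next location, offset from the actor's root, and sets control rotation.
; Reaching the last entry sets Final, so the following call loads M_MainHub_New.
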(event EventBeginPlay
  (if (Variables|Default|Getactive)
    (bind _asbp_main_character (Utilities|Casting|CastToBP_MainCharacter (Game|GetPlayerCharacter 0)))
    (Variables|/Game/Arxcana/Core/MainCharacter/BP_MainCharacter.BP_MainCharacter_C|SetwarpManager _asbp_main_character self)
    (Variables|Default|SetcurrWarpIndex -1)
    (CallFunction|WarptoNextLevel)))

(fn ConstructionScript)

(fn WarptoNextLevel
  (bind _currwarpindex (Variables|Default|GetcurrWarpIndex))
  (if (Variables|Default|Getfinal)
    (Game|OpenLevel(byObjectReference) "/Game/Arxcana/Maps/M_MainHub_New.M_MainHub_New")
    (else
      (bind _result (Math|Integer|IncrementInt _currwarpindex)
        (:%20%20
          (if (Utilities|Array|IsValidIndex (Variables|Default|GetwarpLocations) _result)
            (if (not (== _currwarpindex (- (Utilities|Array|Length (Variables|Default|GetwarpLocations)) 1)))
              _
              (else
                (Variables|Default|Setfinal true)))
            (Transformation|SetActorLocationAndRotation (Game|GetPlayerCharacter 0) (+ (Transformation|GetWorldLocation (Variables|Default|GetDefaultSceneRoot)) (.location (Utilities|Array|Get(acopy) (Variables|Default|GetwarpLocations) _result))) "0, 0, 0" false true)
            (Pawn|SetControlRotation (Game|GetPlayerController 0) (.rotation (Utilities|Array|Get(acopy) (Variables|Default|GetwarpLocations) _result)))))))))