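; BP_DistractTrap is a trap that, when activated, lures a BP_AIZombie by adding the trap's location to its patrol points.
; Its trigger box stores the overlapping zombie and toggles the player HUD's yellow indicator on begin and end overlap.
; ActivateTrap acts only on that single stored zombie.
; End overlap clears it without checking which actor left and leaves Overlapping set to true.
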(event OnComponentBeginOverlap(TriggerBox)
  (params (OverlappedComponent :type Primitive%20Component%20Object%20Reference) (OtherActor :type Actor%20Object%20Reference) (OtherComp :type Primitive%20Component%20Object%20Reference) (OtherBodyIndex :type Integer) (bFromSweep :type Boolean) (SweepResult :type Hit%20Result%20Structure%20%28by%20ref%29))
  (Variables|Default|Setoverlapping true)
  (bind _asbp_aizombie (Utilities|Casting|CastToBP_AIZombie OtherActor))
  (Variables|Default|SetoverlappingActor _asbp_aizombie)
  (Development|PrintString "Begin Overlap")
  (bind _asbp_main_character (Utilities|Casting|CastToBP_MainCharacter (Game|GetPlayerCharacter 0)))
  (Default|EnableYellow (Variables|/Game/Debug/Blueprints/Characters/BP_MainCharacter.BP_MainCharacter_C|GetplayerHUD _asbp_main_character)))

(event OnComponentEndOverlap(TriggerBox)
  (params (OverlappedComponent :type Primitive%20Component%20Object%20Reference) (OtherActor :type Actor%20Object%20Reference) (OtherComp :type Primitive%20Component%20Object%20Reference) (OtherBodyIndex :type Integer))
  (Variables|Default|Setoverlapping true)
  (Variables|Default|SetoverlappingActor 0)
  (Development|PrintString "End Overlap")
  (bind _asbp_main_character (Utilities|Casting|CastToBP_MainCharacter (Game|GetPlayerCharacter 0)))
  (Default|DisableYellow (Variables|/Game/Debug/Blueprints/Characters/BP_MainCharacter.BP_MainCharacter_C|GetplayerHUD _asbp_main_character)))

(event Custom|ActivateTrap
  (bind _overlappingactor (Variables|Default|GetoverlappingActor))
  (Utilities|IsValid _overlappingactor
    (:Is%20Valid
      (Development|PrintString "DISTRACT TRAP ACTIVATED!")
      (Default|AddPatrolPoint _overlappingactor (Transformation|GetActorLocation)))))

(fn ConstructionScript)