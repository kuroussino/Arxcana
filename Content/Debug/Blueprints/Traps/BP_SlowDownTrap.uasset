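; BP_SlowDownTrap is a triggered trap that temporarily slows a BP_AIZombie.
; Its TriggerBox stores an entering zombie and enables the player HUD's blue indicator.
; Any end overlap disables the indicator and clears the stored zombie five seconds later.
; ActivateTrap, not called within this graph, lowers the stored zombie's MaxWalkSpeed, waits five seconds, then restores the saved speed, with debug prints.
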(event OnComponentBeginOverlap(TriggerBox)
  (params (OverlappedComponent :type Primitive%20Component%20Object%20Reference) (OtherActor :type Actor%20Object%20Reference) (OtherComp :type Primitive%20Component%20Object%20Reference) (OtherBodyIndex :type Integer) (bFromSweep :type Boolean) (SweepResult :type Hit%20Result%20Structure%20%28by%20ref%29))
  (Variables|Default|Setoverlapping true)
  (bind _asbp_aizombie (Utilities|Casting|CastToBP_AIZombie OtherActor))
  (Variables|Default|SetoverlappingActor _asbp_aizombie)
  (Development|PrintString "Begin Overlap")
  (bind _asbp_main_character (Utilities|Casting|CastToBP_MainCharacter (Game|GetPlayerCharacter 0)))
  (Default|EnableBlue (Variables|/Game/Debug/Blueprints/Characters/BP_MainCharacter.BP_MainCharacter_C|GetplayerHUD _asbp_main_character)))

(event OnComponentEndOverlap(TriggerBox)
  (params (OverlappedComponent :type Primitive%20Component%20Object%20Reference) (OtherActor :type Actor%20Object%20Reference) (OtherComp :type Primitive%20Component%20Object%20Reference) (OtherBodyIndex :type Integer))
  (Variables|Default|Setoverlapping false)
  (Development|PrintString "End Overlap")
  (bind _asbp_main_character (Utilities|Casting|CastToBP_MainCharacter (Game|GetPlayerCharacter 0)))
  (Default|DisableBlue (Variables|/Game/Debug/Blueprints/Characters/BP_MainCharacter.BP_MainCharacter_C|GetplayerHUD _asbp_main_character))
  (Utilities|FlowControl|Delay 5.0)
  (Variables|Default|SetoverlappingActor 0))

(event Custom|ActivateTrap
  (bind _overlappingactor (Variables|Default|GetoverlappingActor))
  (bind _charactermovement (Variables|/Script/Engine.Character|GetCharacterMovement _overlappingactor))
  (Utilities|IsValid _overlappingactor
    (:Is%20Valid
      (Variables|Default|SetdefaultWalkSpeed (Class|MovementComponent|GetMaxSpeed _charactermovement))
      (Variables|/Script/Engine.CharacterMovementComponent|SetMaxWalkSpeed _charactermovement (Variables|Default|GetslowedWalkSpeed))
      (Development|PrintString "SLOW DOWN TRAP ACTIVATED!")
      (Utilities|FlowControl|Delay 5.0)
      (Variables|/Script/Engine.CharacterMovementComponent|SetMaxWalkSpeed _charactermovement (Variables|Default|GetdefaultWalkSpeed))
      (Development|PrintString "SLOW DOWN TRAP FINISHED ITS EFFECT!"))))

(fn ConstructionScript)