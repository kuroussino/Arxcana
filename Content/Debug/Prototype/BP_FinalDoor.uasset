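; Prototype puzzle door that opens when its linked torches match a required lit/unlit pattern.
; On BeginPlay it binds a check to every torch in the enable and disable lists.
; The check reads each torch's point light visibility, requiring all of the first list lit and all of the second unlit.
; A match plays a timeline, scaled by TrackTime, that raises the left, middle and right panels.
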(event Custom|CheckToches
  (bind _allactive (CallFunction|CheckTorches))
  (if _allactive
    (Components|Timeline|SetPlayRate (Variables|Default|GetOpenDoor) (/ 1.0 (Variables|Default|GettrackTime)))
    (bind _lerpvalue (Timeline|OpenDoor PlayFromStart)
      (:Update
        (Utilities|FlowControl|Sequence
          (:then_0
            (Transformation|SetRelativeLocation (Variables|Default|Getleft) (Math|Vector|Lerp(Vector) "-200.000000,0.000000,0.000000" "-200.000000,0.000000,350.000000" _lerpvalue) false false))
          (:then_1
            (Transformation|SetRelativeLocation (Variables|Default|Getmiddle) (Math|Vector|Lerp(Vector) "0, 0, 0" "0.000000,0.000000,350.000000" _lerpvalue) false false))
          (:then_2
            (Transformation|SetRelativeLocation (Variables|Default|Getright) (Math|Vector|Lerp(Vector) "200.000000,0.000000,0.000000" "200.000000,0.000000,350.000000" _lerpvalue) false false)))))))

(event EventBeginPlay
  (for _array_element (Variables|Default|GettorchesToEnable)
    (EventDispatchers|BindEventtoActiveCheck _array_element (delegate Custom|CheckToches)))
  (for _array_element_2 (Variables|Default|GettorchesToDisable)
    (EventDispatchers|BindEventtoActiveCheck _array_element_2 (delegate Custom|CheckToches))))

(fn ConstructionScript)

(fn CheckTorches
  (Variables|Default|SetactiveTorches 0)
  (Variables|Default|SetdisabledTorches 0)
  (for _array_element (Variables|Default|GettorchesToEnable)
    (if (Rendering|IsVisible (Variables|/Game/Debug/Prototype/BP_Debug_LaserSensorActivationTest.BP_Debug_LaserSensorActivationTest_C|GetPointLight _array_element))
      (Math|Integer|IncrementInt (Variables|Default|GetactiveTorches))))
  (for _array_element_2 (Variables|Default|GettorchesToDisable)
    (if (not (Rendering|IsVisible (Variables|/Game/Debug/Prototype/BP_Debug_LaserSensorActivationTest.BP_Debug_LaserSensorActivationTest_C|GetPointLight _array_element_2)))
      (Math|Integer|IncrementInt (Variables|Default|GetdisabledTorches))))
  (if (and (== (Variables|Default|GetactiveTorches) (Utilities|Array|Length (Variables|Default|GettorchesToEnable))) (== (Variables|Default|GetdisabledTorches) (Utilities|Array|Length (Variables|Default|GettorchesToDisable))))
    (return true)
    (else
      (return false))))