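; The Chariot tarot card for the puzzle game, which lets the player place a cement block while the card is positioned.
; ToggleFunction ties guide display to the Positioned state, and Tick spawns, moves or destroys the guide accordingly.
; A camera-forward line trace drives the guide's location, ignoring the guide itself once it exists.
; PlaceBlock swaps the guide for a BP_CementBlock when its position is legal.
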(event EventBeginPlay
  (|CallParentFunction)
  (Variables|Default|SetCardType "NewEnumerator2")
  (Collision|SetCollisionEnabled (Variables|Default|GetBox) "NoCollision"))

(event Collision|EventActorBeginOverlap
  (params (OtherActor :type Actor%20Object%20Reference))
  (|CallParentFunction OtherActor) ; This node is disabled and will not be called.\nDrag off pins to build functionality.
)

(event EventTick
  (params (DeltaSeconds :type Float%20%28single-precision%29))
  (|CallParentFunction DeltaSeconds)
  (Utilities|FlowControl|Delay 0.025)
  (if (Variables|Default|GetneedShowGuide)
    (CallFunction|ShowGuide)
    (elif (Utilities|IsValid (Variables|Default|GetcurrGuide))
      (CallFunction|DestroyGuide))))

(event EventDestroyed
  (CallFunction|DestroyGuide))

(fn ConstructionScript
  (|CallParentFunction))

(fn ToggleFunction
  (if (Variables|Default|Getpositioned)
    (Variables|Default|SetneedShowGuide true)
    (else
      (Variables|Default|SetneedShowGuide false))))

(fn ShowGuide
  (bind _returnvalue (Game|GetPlayerCameraManager 0))
  (bind _returnvalue_2 (Game|GetPlayerCameraManager 0))
  (bind _returnvalue_3 (Camera|GetCameraLocation _returnvalue))
  (bind _returnvalue_4 (Camera|GetCameraLocation _returnvalue_2))
  (if (Utilities|IsValid (Variables|Default|GetcurrGuide))
    (bind (_outhit _returnvalue_5) (Collision|LineTraceByChannel _returnvalue_3 (+ _returnvalue_3 (* (Math|Vector|GetForwardVector (Camera|GetCameraRotation _returnvalue)) (Variables|Default|GetlineTraceDistance))) "TraceTypeQuery1" false (Utilities|Array|MakeArray (Variables|Default|GetcurrGuide)) "ForDuration"))
    (if _returnvalue_5
      (Transformation|SetActorLocation (Variables|Default|GetcurrGuide) (.Location (Collision|BreakHitResult _outhit)) false false)
      (else
        (Actor|DestroyActor (Variables|Default|GetcurrGuide))
        (Variables|Default|SetcurrGuide 0)))
    (else
      (bind (_outhit_2 _returnvalue_6) (Collision|LineTraceByChannel _returnvalue_4 (+ _returnvalue_4 (* (Math|Vector|GetForwardVector (Camera|GetCameraRotation _returnvalue_2)) (Variables|Default|GetlineTraceDistance))) "TraceTypeQuery1" false 0 "ForDuration"))
      (if _returnvalue_6
        (bind _returnvalue_7 (Game|SpawnActorfromClass "/Game/TarotPuzzleGame/Placeables/BP_CementBlockGuide.BP_CementBlockGuide_C" (Math|Conversions|ToTransform(Vector) (.Location (Collision|BreakHitResult _outhit_2))) "Undefined" "MultiplyWithRoot" 0 0))
        (Variables|Default|SetcurrGuide _returnvalue_7)))))

(fn PlaceBlock
  (if (Math|Boolean|ANDBoolean (Variables|Default|Getpositioned) (Utilities|IsValid (Variables|Default|GetcurrGuide)) (Variables|/Game/TarotPuzzleGame/Placeables/BP_CementBlockGuide.BP_CementBlockGuide_C|GetlegalPosition (Variables|Default|GetcurrGuide)))
    (Game|SpawnActorfromClass "/Game/TarotPuzzleGame/Placeables/BP_CementBlock.BP_CementBlock_C" (Transformation|GetActorTransform (Variables|Default|GetcurrGuide)) "AdjustIfPossibleButAlwaysSpawn" "MultiplyWithRoot" 0 0)
    (Actor|DestroyActor (Variables|Default|GetcurrGuide))
    (Variables|Default|SetcurrGuide 0)))

(fn DestroyGuide
  (Utilities|IsValid (Variables|Default|GetcurrGuide)
    (:Is%20Valid
      (Actor|DestroyActor (Variables|Default|GetcurrGuide))
      (Variables|Default|SetcurrGuide 0))))