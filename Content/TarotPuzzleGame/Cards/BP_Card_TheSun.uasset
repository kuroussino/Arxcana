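; The Sun tarot card in the puzzle game, a card actor that acts as a flashlight and can fire a laser beam.
; Toggling the beam on hides the point light and spawns a laser emitter at the beam spawn point, aimed along the camera's rotation and attached there.
; Toggling it off stops and destroys that emitter and restores the light.
; BeginPlay sets the card type, and destroying the card switches the light off.
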(event EventBeginPlay
  (|CallParentFunction)
  (Variables|Default|SetCardType "NewEnumerator0"))

(event Collision|EventActorBeginOverlap
  (params (OtherActor :type Actor%20Object%20Reference))
  (|CallParentFunction OtherActor) ; This node is disabled and will not be called.\nDrag off pins to build functionality.
)

(event EventTick
  (params (DeltaSeconds :type Float%20%28single-precision%29))
  (|CallParentFunction DeltaSeconds) ; This node is disabled and will not be called.\nDrag off pins to build functionality.
)

(event EventDestroyed
  (CallFunction|SetFlashlightVisibility false))

(fn ConstructionScript
  (|CallParentFunction))

(fn SetFlashlightVisibility
  (params (active :type Boolean))
  (bind _pointlight (Variables|Default|GetPointLight))
  (if active
    (Rendering|SetVisibility _pointlight true false)
    (else
      (Rendering|SetVisibility _pointlight false false))))

(fn ToggleFunction
  (params (beam :type Boolean))
  (bind _beamspawnpoint (Variables|Default|GetBeamSpawnPoint))
  (if beam
    (CallFunction|SetFlashlightVisibility false)
    (bind _returnvalue (Game|SpawnActorfromClass "/Game/TarotPuzzleGame/Core/LaserSystem/BP_LaserEmitter_Card_TheSun.BP_LaserEmitter_Card_TheSun_C" (Math|Transform|MakeTransform (Transformation|GetWorldLocation _beamspawnpoint) (Camera|GetCameraRotation (Game|GetPlayerCameraManager 0)) "1.000000,1.000000,1.000000") "Undefined" "MultiplyWithRoot" 0 0))
    (bind _output_get (Variables|Default|SetcurrentBeam _returnvalue))
    (Transformation|AttachComponentToComponent _output_get _beamspawnpoint "None" "KeepWorld" "KeepWorld" "KeepWorld" true)
    (Variables|/Game/TarotPuzzleGame/Core/LaserSystem/BP_LaserEmitter_Card_TheSun.BP_LaserEmitter_Card_TheSun_C|Setemitting (Variables|Default|GetcurrentBeam) true)
    (else
      (Utilities|IsValid (Variables|Default|GetcurrentBeam)
        (:Is%20Valid
          (Default|StopBeam (Variables|Default|GetcurrentBeam))
          (Variables|/Game/TarotPuzzleGame/Core/LaserSystem/BP_LaserEmitter_Card_TheSun.BP_LaserEmitter_Card_TheSun_C|Setemitting (Variables|Default|GetcurrentBeam) false)
          (Actor|DestroyActor (Variables|Default|GetcurrentBeam))
          (CallFunction|SetFlashlightVisibility true)
          (Variables|Default|SetcurrentBeam 0))))))