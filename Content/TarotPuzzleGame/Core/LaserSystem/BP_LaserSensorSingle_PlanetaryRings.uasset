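; Laser sensor for the tarot puzzle game that cycles a planetary rings actor through configured ring sets.
; An on signal to ToggleState sets a Toggling flag and, after two seconds, applies the current set and advances the wrapping index if the flag is still set.
; Tick clears the flag through a short repeating Delay, so the change requires the signal to still be arriving when the wait ends.
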(event EventBeginPlay
  (Variables|Default|SetcurrStateIndex 0))

(event Collision|EventActorBeginOverlap
  (params (OtherActor :type Actor%20Object%20Reference)))

(event EventTick
  (params (DeltaSeconds :type Float%20%28single-precision%29))
  (Utilities|FlowControl|Delay 0.2)
  (Variables|Default|Settoggling false))

(event EventToggleState
  (params (On/Off :type Boolean))
  (if On/Off
    (Variables|Default|Settoggling true)
    (Utilities|FlowControl|Delay 2.0)
    (if (Variables|Default|Gettoggling)
      (Default|ChangeRingsState (Variables|Default|GetplanetaryRef) (Utilities|Struct|BreakSTR_RingSet (Utilities|Array|Get(acopy) (Variables|Default|GetringSets) (Variables|Default|GetcurrStateIndex))))
      (bind _result (Math|Integer|IncrementInt (Variables|Default|GetcurrStateIndex))
        (:%20%20
          (if (> _result (- (Utilities|Array|Length (Variables|Default|GetringSets)) 1))
            (Variables|Default|SetcurrStateIndex 0)))))))

(fn ConstructionScript)