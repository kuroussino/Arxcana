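; BP_PuzzleTrigger is a floating card pickup that unlocks a tarot card and can toggle puzzle lights.
; Two timelines chain into each other to bob the mesh up and down.
; When the player overlaps the box, it enables its CardType in the HUD's radial inventory.
; If NeedsToTriggerPuzzle is set, it sends ToggleStateMessage to each entry in Lights, then destroys itself either way.
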(event OnComponentBeginOverlap(Box)
  (params (OverlappedComponent :type Primitive%20Component%20Object%20Reference) (OtherActor :type Actor%20Object%20Reference) (OtherComp :type Primitive%20Component%20Object%20Reference) (OtherBodyIndex :type Integer) (bFromSweep :type Boolean) (SweepResult :type Hit%20Result%20Structure%20%28by%20ref%29))
  (bind _returnvalue (Game|GetPlayerCharacter 0))
  (if (== OtherActor _returnvalue)
    (bind _asbp_main_character (Utilities|Casting|CastToBP_MainCharacter _returnvalue))
    (Default|EnableCard (Variables|/Game/TarotPuzzleGame/Core/UI/WBP_HUD.WBP_HUD_C|GetBPW_RadialInventory (Variables|/Game/TarotPuzzleGame/Core/MainCharacter/BP_MainCharacter.BP_MainCharacter_C|GetplayerHUD _asbp_main_character)) (Variables|Default|GetcardType))
    (if (Variables|Default|GetneedsToTriggerPuzzle)
      (CallFunction|ToggleTorches (Variables|Default|Geton/off)))
    (Actor|DestroyActor)))

(event Collision|EventActorBeginOverlap
  (params (OtherActor :type Actor%20Object%20Reference)))

(event EventTick
  (params (DeltaSeconds :type Float%20%28single-precision%29)))

(event EventBeginPlay
  (bind _0_1 (Timeline|FloatingUp Play)
    (:Update
      (Transformation|SetRelativeLocation (Variables|Default|GetStaticMesh) (Math|Vector|MakeVector 0.0 0.0 (* _0_1 1e+01)) false false))
    (:Finished
      (bind _1_0 (Timeline|FloatingDown PlayFromStart)
        (:Update
          (Transformation|SetRelativeLocation (Variables|Default|GetStaticMesh) (Math|Vector|MakeVector 0.0 0.0 (* _1_0 1e+01)) false false))
        (:Finished
          (Timeline|FloatingUp PlayFromStart))))))

(fn ConstructionScript)

(fn ToggleTorches
  (params (on/off :type Boolean))
  (for _array_element (Variables|Default|Getlights)
    (Class|BPISetState|ToggleState(Message) _array_element on/off)))