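; BP_CementBlockGuide is a placement guide actor for a cement block, showing whether its current position is legal.
; BeginPlay creates a dynamic material from MM_CementBlockGuide, whose emissive color switches between legal and illegal colors as the Box begins or ends overlaps, also setting LegalPosition.
; Tick, through a short Delay, yaws the actor along the direction from the player character to itself.
; Overlaps are not counted, so any single end overlap restores the legal state.
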(event OnComponentBeginOverlap(Box)
  (params (OverlappedComponent :type Primitive%20Component%20Object%20Reference) (OtherActor :type Actor%20Object%20Reference) (OtherComp :type Primitive%20Component%20Object%20Reference) (OtherBodyIndex :type Integer) (bFromSweep :type Boolean) (SweepResult :type Hit%20Result%20Structure%20%28by%20ref%29))
  (Rendering|Material|SetVectorParameterValue (Variables|Default|GetguideMaterial) "Emissive Color" (Math|Conversions|ToLinearColor(Color) (Variables|Default|GetillegalPosColor)) :!class /Script/Engine.MaterialInstanceDynamic)
  (Variables|Default|SetlegalPosition false))

(event OnComponentEndOverlap(Box)
  (params (OverlappedComponent :type Primitive%20Component%20Object%20Reference) (OtherActor :type Actor%20Object%20Reference) (OtherComp :type Primitive%20Component%20Object%20Reference) (OtherBodyIndex :type Integer))
  (Rendering|Material|SetVectorParameterValue (Variables|Default|GetguideMaterial) "Emissive Color" (Math|Conversions|ToLinearColor(Color) (Variables|Default|GetlegalPosColor)) :!class /Script/Engine.MaterialInstanceDynamic)
  (Variables|Default|SetlegalPosition true))

(event EventBeginPlay
  (bind _returnvalue (Rendering|Material|CreateDynamicMaterialInstance (Variables|Default|GetCementBlockGuide) 0 "/Game/TarotPuzzleGame/Art/Props/MM_CementBlockGuide.MM_CementBlockGuide" "None" :!class /Script/Engine.PrimitiveComponent))
  (Variables|Default|SetguideMaterial _returnvalue))

(event Collision|EventActorBeginOverlap
  (params (OtherActor :type Actor%20Object%20Reference)))

(event EventTick
  (params (DeltaSeconds :type Float%20%28single-precision%29))
  (Utilities|FlowControl|Delay 0.025)
  (Transformation|SetActorRotation (Math|Rotator|MakeRotator 0.0 0.0 (.yaw (Math|Rotator|FindLookatRotation (Transformation|GetActorLocation (Game|GetPlayerCharacter 0)) (Transformation|GetActorLocation))))))

(fn ConstructionScript)